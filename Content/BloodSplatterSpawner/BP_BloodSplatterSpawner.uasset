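; BP_BloodSplatterSpawner is a one-shot actor that places a blood splatter on a nearby surface.
; Five seconds after BeginPlay, it runs a stationary sphere trace on Visibility at its root location, sized by SplatterRange, with persistent debug drawing.
; It spawns BP_BloodSplatter at the impact point aligned to the surface normal, plays a splat sound, then destroys itself, without checking for a hit.
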(event EventBeginPlay
  (bind _defaultsceneroot (Variables|Default|GetDefaultSceneRoot))
  (bind _relativelocation (Variables|/Script/Engine.SceneComponent|GetRelativeLocation _defaultsceneroot))
  (Utilities|FlowControl|Delay 5.0)
  (bind _outhit (Collision|SphereTraceByChannel _relativelocation _relativelocation (Variables|Default|GetSplatterRange) "TraceTypeQuery1" false 0 "Persistent" true "(R=1.000000,G=0.000000,B=0.783848,A=1.000000)" "(R=1.000000,G=0.030547,B=0.000000,A=1.000000)" 0.0))
  (bind _returnvalue (Game|SpawnActorfromClass "/Game/BloodSplatterSpawner/BP_BloodSplatter.BP_BloodSplatter_C" (Math|Conversions|ToTransform(Vector) (.ImpactPoint (Collision|BreakHitResult _outhit))) "Undefined" "MultiplyWithRoot" 0 0))
  (Transformation|SetActorRotation _returnvalue (Math|Rotator|MakeRotfromZ (.ImpactNormal (Collision|BreakHitResult _outhit))))
  (Audio|PlaySoundatLocation "/Game/SFXs/Splat_SFX.Splat_SFX" (.ImpactPoint (Collision|BreakHitResult _outhit)) "0, 0, 0" 1.0 1.0 0.0 0 0 0 0)
  (Actor|DestroyActor))

(fn ConstructionScript)