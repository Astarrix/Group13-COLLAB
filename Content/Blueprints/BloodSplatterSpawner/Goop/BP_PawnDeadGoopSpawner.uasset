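; Short-lived spawner for a blood explosion, apparently for pawn death, that fires on BeginPlay and destroys itself one second later.
; Plays a Niagara burst and sound, then scatters BP_BloodSplatter actors using randomly offset sphere traces that ignore BP_PawnDeadGoop actors.
; Each splatter is aligned to its impact normal and has its cleaned event bound.
; An object-type sphere trace at the splatter radius triggers a camera shake on any hit, intended for nearby players.
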(event Custom|Splatter
  (bind _splatterspacing (Variables|Default|GetSplatterSpacing))
  (bind _returnvalue (* _splatterspacing -1.0))
  ;[1 0 0] Splatter Function
  (Niagara|SpawnSystemAttached "/Game/VFX/NS_BloodExplosion.NS_BloodExplosion" (Variables|Default|GetNs_Blood) "None" "0, 0, 0" "0, 0, 0" "KeepRelativeOffset" true)
  (Audio|PlaySoundatLocation "/Game/Audio/SFXs/BloodSplat_Explode.BloodSplat_Explode" (Variables|/Script/Engine.SceneComponent|GetRelativeLocation (Variables|Default|GetDefaultSceneRoot)) "0, 0, 0" 1.0 1.0 0.0 0 0 0 0)
  (bind _output_get (Variables|Default|SetNumOfSplatters (Math|Random|RandomInteger (Variables|Default|GetMaxNumOfSplatters))))
  (for _index (range (Variables|Default|GetMinNumOfSplatters) _output_get)
    (Variables|Default|SetOffset (Math|Vector|MakeVector (Math|Random|RandomFloatinRange _returnvalue _splatterspacing) (Math|Random|RandomFloatinRange _returnvalue _splatterspacing) (Math|Random|RandomFloatinRange _returnvalue _splatterspacing)))
    (bind _outactors (Actor|GetAllActorsOfClass "/Game/Blueprints/BloodSplatterSpawner/Goop/BP_PawnDeadGoop.BP_PawnDeadGoop_C"))
    (bind _outhit (Collision|SphereTraceByChannel (+ (Variables|/Script/Engine.SceneComponent|GetRelativeLocation (Variables|Default|GetDefaultSceneRoot)) (Variables|Default|GetOffset)) (+ (Variables|/Script/Engine.SceneComponent|GetRelativeLocation (Variables|Default|GetDefaultSceneRoot)) (Variables|Default|GetOffset)) (Variables|Default|GetSplatterRange) "TraceTypeQuery1" false _outactors "None" true "(R=1.000000,G=0.000000,B=0.783848,A=1.000000)" "(R=1.000000,G=0.030547,B=0.000000,A=1.000000)" 0.0))
    (bind _returnvalue_2 (Game|SpawnActorfromClass "/Game/Blueprints/BloodSplatterSpawner/BP_BloodSplatter.BP_BloodSplatter_C" (Math|Conversions|ToTransform(Vector) (.ImpactPoint (Collision|BreakHitResult _outhit))) "Undefined" "MultiplyWithRoot" 0 0))
    (EventDispatchers|BindEventtoOnSplatterCleaned _returnvalue_2 (EventDispatchers|CreateEvent (Variables|Default|GetPlayer) :!event AddSplatterMoney))
    (Transformation|SetActorRotation _returnvalue_2 (Math|Rotator|MakeRotfromZ (.ImpactNormal (Collision|BreakHitResult _outhit)))))
  (Utilities|FlowControl|Delay 1.0)
  (Actor|DestroyActor))

(event Custom|Screnn%20Shake
  (bind _defaultsceneroot (Variables|Default|GetDefaultSceneRoot))
  (bind _relativelocation (Variables|/Script/Engine.SceneComponent|GetRelativeLocation _defaultsceneroot))
  ;[1 0 0] Shakes Players Screen if they are too close to blood splatter explosion
  (bind _returnvalue (Collision|SphereTraceForObjects _relativelocation _relativelocation (Variables|Default|GetSplatterRange) (Variables|Default|GetObject%20Types) false 0 "ForOneFrame" true "(R=0.554122,G=1.000000,B=0.000000,A=1.000000)"))
  (if _returnvalue
    (CallFunction|CameraShakewithOptions (Game|GetPlayerCameraManager 0) true 7 7 7)))

(event EventBeginPlay
  ;[1 0 0] Spawns on Begin Play Atm to debug
  (bind _asbp_character (Utilities|Casting|CastToBP_Character (Game|GetPlayerCharacter 0)))
  (Variables|Default|SetPlayer _asbp_character)
  (CallFunction|Splatter)
  (CallFunction|ScrennShake))

(fn ConstructionScript)