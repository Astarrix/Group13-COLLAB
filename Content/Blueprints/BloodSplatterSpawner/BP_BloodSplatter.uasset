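; BP_BloodSplatter is a cleanable blood decal actor that gets a random roll when constructed.
; Both AnyDamage and a once-only AttemptWash lead to the same cleanup: play a 2D sound, destroy the actor and call OnSplatterCleaned.
; Washing also requests a short decal fade first, though the destroy follows without waiting for it.
; AttemptPickUpWeapon always refuses pickup.
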(event EventAttemptWash
  (Utilities|FlowControl|DoOnce false
    (:Completed
      (Rendering|Components|Decal|SetFadeOut (Variables|Default|GetDecal) 0.0 0.1 true)
      (Audio|SpawnSound2D "/Game/Audio/SFXs/BloodSplat_Cleared.BloodSplat_Cleared" 1.0 1.0 0.0 0)
      (Actor|DestroyActor)
      (Default|CallOnSplatterCleaned))))

(event Game|Damage|EventAnyDamage
  (params (Damage :type Float%20%28single-precision%29) (DamageType :type Damage%20Type%20Object%20Reference) (InstigatedBy :type Controller%20Object%20Reference) (DamageCauser :type Actor%20Object%20Reference))
  ;[1 1 1] Can shoot them on Ground With This
  (Audio|SpawnSound2D "/Game/Audio/SFXs/BloodSplat_Cleared.BloodSplat_Cleared" 1.0 1.0 0.0 0)
  (Actor|DestroyActor)
  (Default|CallOnSplatterCleaned))

(fn ConstructionScript
  (Transformation|AddRelativeRotation (Variables|Default|GetDecal) (Math|Rotator|MakeRotator (Math|Random|RandomFloatinRange 0.0 3.6e+02) 0.0 0.0) false false))

(fn AttemptPickUpWeapon
  (params (IsLeftArm :type Boolean))
  (return false 0))