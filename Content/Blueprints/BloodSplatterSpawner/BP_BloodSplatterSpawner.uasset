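; Blood splatter spawner actor that plays an explosion effect and sound, scatters BP_BloodSplatter actors on nearby surfaces, then destroys itself after a delay.
; For a random count, it runs zero-length sphere traces at random offsets around the root's relative location, ignoring existing splatters.
; Each splatter spawns at the impact point, aligned to its normal, without checking for a hit.
; BeginPlay auto-triggers Splatter after a delay for debugging, with persistent trace drawing.
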(event Custom|Splatter
  (bind _splatterspacing (Variables|Default|GetSplatterSpacing))
  (bind _returnvalue (* _splatterspacing -1.0))
  ;[1 0 0] Splatter Function
  (Niagara|SpawnSystemAttached "/Game/VFX/NS_BloodExplosion.NS_BloodExplosion" (Variables|Default|GetNs_Blood) "None" "0, 0, 0" "0, 0, 0" "KeepRelativeOffset" true)
  (Audio|PlaySoundatLocation "/Game/Audio/SFXs/BloodSplat_Explode.BloodSplat_Explode" (Variables|/Script/Engine.SceneComponent|GetRelativeLocation (Variables|Default|GetDefaultSceneRoot)) "0, 0, 0" 1.0 1.0 0.0 0 0 0 0)
  (bind _output_get (Variables|Default|SetNumOfSplatters (Math|Random|RandomInteger (Variables|Default|GetMaxNumOfSplatters))))
  (for _index (range (Variables|Default|GetMinNumOfSplatters) _output_get)
    (Variables|Default|SetOffset (Math|Vector|MakeVector (Math|Random|RandomFloatinRange _returnvalue _splatterspacing) (Math|Random|RandomFloatinRange _returnvalue _splatterspacing) (Math|Random|RandomFloatinRange _returnvalue _splatterspacing)))
    (bind _outactors (Actor|GetAllActorsOfClass "/Game/Blueprints/BloodSplatterSpawner/BP_BloodSplatter.BP_BloodSplatter_C"))
    (bind _outhit (Collision|SphereTraceByChannel (+ (Variables|/Script/Engine.SceneComponent|GetRelativeLocation (Variables|Default|GetDefaultSceneRoot)) (Variables|Default|GetOffset)) (+ (Variables|/Script/Engine.SceneComponent|GetRelativeLocation (Variables|Default|GetDefaultSceneRoot)) (Variables|Default|GetOffset)) (Variables|Default|GetSplatterRange) "TraceTypeQuery1" false _outactors "Persistent" true "(R=1.000000,G=0.000000,B=0.783848,A=1.000000)" "(R=1.000000,G=0.030547,B=0.000000,A=1.000000)" 0.0))
    (bind _returnvalue_2 (Game|SpawnActorfromClass "/Game/Blueprints/BloodSplatterSpawner/BP_BloodSplatter.BP_BloodSplatter_C" (Math|Conversions|ToTransform(Vector) (.ImpactPoint (Collision|BreakHitResult _outhit))) "Undefined" "MultiplyWithRoot" 0 0))
    (Transformation|SetActorRotation _returnvalue_2 (Math|Rotator|MakeRotfromZ (.ImpactNormal (Collision|BreakHitResult _outhit)))))
  (Utilities|FlowControl|Delay 5.0)
  (Actor|DestroyActor))

(event EventBeginPlay
  ;[1 1 1] Spawns on Begin Play Atm to debug
  (Utilities|FlowControl|Delay 3.0)
  (CallFunction|Splatter))

(fn ConstructionScript)