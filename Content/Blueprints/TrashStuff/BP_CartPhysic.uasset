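; BP_CartPhysic is a damageable cart that reacts to hits and is destroyed when its health runs out.
; Each AnyDamage event plays a hit sound, subtracts from Health and spawns a trash explosion Niagara effect on the Cart component, tinted by ParticleColour.
; At zero health or below it plays a death sound, spawns a second explosion and destroys itself after a short delay.
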(event Game|Damage|EventAnyDamage
  (params (Damage :type Float%20%28single-precision%29) (DamageType :type Damage%20Type%20Object%20Reference) (InstigatedBy :type Controller%20Object%20Reference) (DamageCauser :type Actor%20Object%20Reference))
  (Audio|PlaySound2D "/Game/Audio/SFXs/Can_Hit.Can_Hit" 1.0 1.0 0.0 0 0)
  (Variables|Default|SetHealth (- (Variables|Default|GetHealth) Damage))
  (bind _returnvalue (Niagara|SpawnSystemAttached "/Game/VFX/NS_TrashExplosion.NS_TrashExplosion" (Variables|Default|GetCart) "None" "0, 0, 0" "0, 0, 0" "KeepRelativeOffset" true))
  (Niagara|SetNiagaraVariable(LinearColor) _returnvalue "Colour" (Variables|Default|GetParticleColour))
  (if (<= (Variables|Default|GetHealth) 0.0)
    (Audio|PlaySound2D "/Game/Audio/SFXs/Cart_Dead.Cart_Dead" 1.0 1.0 0.0 0 0)
    (bind _returnvalue_2 (Niagara|SpawnSystemAttached "/Game/VFX/NS_TrashExplosion.NS_TrashExplosion" (Variables|Default|GetCart) "None" "0, 0, 0" "0, 0, 0" "KeepRelativeOffset" true))
    (Niagara|SetNiagaraVariable(LinearColor) _returnvalue_2 "Colour" (Variables|Default|GetParticleColour))
    (Utilities|FlowControl|Delay 0.5)
    (Actor|DestroyActor)))

(fn ConstructionScript)