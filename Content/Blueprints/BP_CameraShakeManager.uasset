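; BP_CameraShakeManager is a camera shake Blueprint that defines Perlin-noise rotation and FOV oscillation.
; Its disconnected logic treats the truncated Scale as a bitfield, unpacking three-bit pitch, yaw and roll amplitudes plus a one-bit FOV flag, then resets ShakeScale.
; PlayShake is empty, so this unpacking never runs, and the FOV amplitude divides by zero.
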(event EventPlayShake
  (params (Scale :type Float%20%28single-precision%29)))