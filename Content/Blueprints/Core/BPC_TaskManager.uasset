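; Blueprint component that sequences the tutorial objectives for a window-washing game, from buying and equipping a washer to cleaning windows.
; On BeginPlay it gets the task list from the player controller's HUD and binds to its task started and completed events.
; Each completed task ID selects the next objective to add, with instruction text that teaches the controls.
; The task-started handler is an empty switch, and some objective calls are left unwired.
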(event Custom|Objective%20Finished
  (params (Unique%20Task%20ID :type Name))
  (switch name Unique%20Task%20ID
    (:BuyWasher
      (CallFunction|AddNewObjective "EquipWasher" "Equip Washer" "Go and walk into that new Washer you just purchased and equip it!"))
    (:EquipWasher
      (CallFunction|AddNewObjective "WalkToBuilding" "Head To The Building" "Get to the building and get ready to clean! Use LMB to activate that Washer!"))
    (:WalkToBuilding
      (CallFunction|AddNewObjective "Clean3Windows" "Clean The Dirty Windows" "Use your Washer toggling between modes with TAB to clean those windows. Press SHIFT to get onto the building and G to switch movement modes!"))))

(event Custom|Objective%20Started
  (params (Unique%20Task%20ID :type Name))
  (switch name Unique%20Task%20ID))

(event EventBeginPlay
  (bind _asbp_player_controller (Utilities|Casting|CastToBP_PlayerController (Game|GetPlayerController 0)))
  (bind _output_get (Variables|Default|SetTask%20Manager (Variables|/Game/UI/NewHUD/UI_HUD.UI_HUD_C|GetUIC_TaskList (Variables|/Game/Blueprints/Core/BP_PlayerController.BP_PlayerController_C|GetHUD _asbp_player_controller))))
  (EventDispatchers|BindEventtoOnTaskStarted _output_get (EventDispatchers|CreateEvent :!event Custom|Objective%20Started))
  (EventDispatchers|BindEventtoOnTaskCompleted _output_get (EventDispatchers|CreateEvent :!event Custom|Objective%20Finished)))