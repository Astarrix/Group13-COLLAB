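; Player character with power-wash spray, directional launch jump, climbing trace helper and single-weapon pickup check.
; PowerWashTrace line-traces from the deprojected mouse position, aims the Niagara spray and foam ring, and paints hit A_Target actors' render targets.
; MechJump launches along a forward-to-up blended vector, and landing triggers a camera shake.
; SetActiveCamera toggles first/third person, mesh owner visibility and levels control pitch, starting in first person.
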(event Custom|JumpLanded
  (params (Hit :type Hit%20Result%20Structure%20%28by%20ref%29))
  (CallFunction|CameraShakewithOptions (Game|GetPlayerCameraManager 0) true 7))

(event Custom|ToggleSpray
  (params (isActive :type Boolean))
  (Components|Activation|SetActive (Variables|Default|GetNS_Spray) isActive false))

(event Custom|BindEvents
  (EventDispatchers|BindEventtoLandedDelegate (EventDispatchers|CreateEvent :!event Custom|JumpLanded)))

(event EventBeginPlay
  (CallFunction|BindEvents)
  (CallFunction|SetActiveCamera false))

(event EventOnLanded
  (params (Hit :type Hit%20Result%20Structure%20%28by%20ref%29))
  (CallFunction|CameraShakewithOptions (Game|GetPlayerCameraManager 0) true 7))

(fn ConstructionScript)

(fn MechJump
  (params (LaunchVelocity :type Float%20%28single-precision%29) (DistanceHeightBias :type Float%20%28single-precision%29))
  (Character|LaunchCharacter (* (Math|Vector|Normalize (Math|Vector|Lerp(Vector) (Transformation|GetActorForwardVector) (Transformation|GetActorUpVector) DistanceHeightBias)) LaunchVelocity) true true)
  (return))

(fn SetActiveCamera
  (params (isThirdPerson :type Boolean))
  (bind _returnvalue (Pawn|GetController))
  (bind _returnvalue_2 (not isThirdPerson))
  (bind _returnvalue_3 (Pawn|GetControlRotation _returnvalue :!class /Script/Engine.Controller))
  (Variables|Default|SetIs%20Third%20Person isThirdPerson)
  ;[1 0.7157 0.01033] Switching cameras
  (Components|Activation|SetActive (Variables|Default|GetThirdPersonCamera) isThirdPerson true)
  (Components|Activation|SetActive (Variables|Default|GetFirstPersonCamera) _returnvalue_2 true)
  (Class|PrimitiveComponent|SetOwnerNoSee (Variables|Character|GetMesh) _returnvalue_2)
  ;[0.3564 0.04092 0.521] Resets rotation to be straight on whenever going to first person
  (Pawn|SetControlRotation _returnvalue (Math|Rotator|MakeRotator (.roll _returnvalue_3) 0.0 (.yaw _returnvalue_3))))

(fn ClimbingLineTrace
  (bind _returnvalue (Transformation|GetActorLocation))
  (bind (_outhit _returnvalue_2) (Collision|LineTraceByChannel _returnvalue (+ _returnvalue (* (Math|Vector|GetForwardVector (Transformation|GetActorRotation)) 1e+02)) "TraceTypeQuery1" false 0 "ForDuration"))
  (return _outhit _returnvalue_2))

(fn PowerWashTrace
  (bind _returnvalue (Game|GetPlayerController 0))
  (bind _ns_foamring (Variables|Default|GetNS_FoamRing))
  (bind (_worldlocation _worlddirection) (Game|Player|ConvertMouseLocationToWorldSpace _returnvalue))
  (bind _outhit (Collision|LineTraceByChannel _worldlocation (+ _worldlocation (* _worlddirection (Math|Float|MakeLiteralFloat 3e+02))) "TraceTypeQuery1" false 0 "None"))
  (Transformation|SetWorldLocation _ns_foamring (.ImpactPoint (Collision|BreakHitResult _outhit)) false false)
  (Transformation|SetRelativeRotation _ns_foamring (Math|Conversions|RotationFromXVector (.Normal (Collision|BreakHitResult _outhit))) false false)
  (Transformation|SetRelativeRotation (Variables|Default|GetNS_Spray) (Math|Rotator|FindLookatRotation _worldlocation (Math|Vector|SelectVector (.ImpactPoint (Collision|BreakHitResult _outhit)) (.TraceEnd (Collision|BreakHitResult _outhit)) (.bBlockingHit (Collision|BreakHitResult _outhit)))) false false)
  (bind _asa_target (Utilities|Casting|CastToA_Target (.HitActor (Collision|BreakHitResult _outhit))))
  (Default|DrawtoRenderTarget _asa_target (.ImpactPoint (Collision|BreakHitResult _outhit)) (Variables|Default|GetSprayRadius)))

(fn AttemptPickUpWeapon
  (if (Variables|Default|GethasWeapon)
    (return false 0)
    (else
      (Variables|Default|SethasWeapon true)
      (return true self))))