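; Game mode Blueprint that bootstraps the single main player on login and exposes a pause event.
; PostLogin stores the BP_PlayerController, then possesses the first placed BP_Character or spawns one at the first PlayerStart, and initialises the controller with the game mode.
; It then creates WBP_MainUI, initialised with character, game mode and controller, and adds it to the viewport.
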(event Custom|Pause%20Game
  (params (Enable%20Pause :type Boolean))
  ;[1 1 1] Pause
  (Game|SetGamePaused Enable%20Pause))

(event EventPostLogin
  (params (NewPlayer :type Player%20Controller%20Object%20Reference))
  (CallFunction|SetupPlayerController NewPlayer)
  (CallFunction|SetupPlayerPawn)
  (CallFunction|SetupMainUI))

(fn ConstructionScript)

(fn SetupPlayerController
  (params (PlayerController :type Player%20Controller%20Object%20Reference))
  (bind _asbp_player_controller (Utilities|Casting|CastToBP_PlayerController PlayerController))
  (Variables|Default|SetMainPlayerController _asbp_player_controller)
  (return))

(fn SetupPlayerPawn
  (bind _mainplayercontroller (Variables|Default|GetMainPlayerController))
  (bind _mainplayercontroller_2 (Variables|Default|GetMainPlayerController))
  (bind _outactors (Actor|GetAllActorsOfClass "/Game/Blueprints/Core/BP_Character.BP_Character_C"))
  (if (> (Utilities|Array|Length _outactors) 0)
    (bind _output_get (Variables|Default|SetMainPlayerCharacter (Utilities|Array|Get(acopy) _outactors)))
    (Pawn|Possess _mainplayercontroller _output_get)
    (Default|Initialise _mainplayercontroller self)
    (return)
    (else
      (bind _outactors_2 (Actor|GetAllActorsOfClass "/Script/Engine.PlayerStart"))
      (bind _returnvalue (Game|SpawnActorfromClass "/Game/Blueprints/Core/BP_Character.BP_Character_C" (Transformation|GetActorTransform (Utilities|Array|Get(acopy) _outactors_2)) "Undefined" "MultiplyWithRoot" 0 0))
      (bind _output_get_2 (Variables|Default|SetMainPlayerCharacter _returnvalue))
      (Pawn|Possess _mainplayercontroller_2 _output_get_2)
      (Default|Initialise _mainplayercontroller_2 self)
      (return))))

(fn SetupMainUI
  (bind _returnvalue (UserInterface|CreateWidget "/Game/UI/HUD/WBP_MainUI.WBP_MainUI_C" (Variables|Default|GetMainPlayerController)))
  (bind _output_get (Variables|Default|SetMain%20UI _returnvalue))
  (Default|Initialise _output_get (Variables|Default|GetMainPlayerCharacter) self (Variables|Default|GetMainPlayerController))
  (UserInterface|Viewport|AddtoViewport (Variables|Default|GetMain%20UI) 0))