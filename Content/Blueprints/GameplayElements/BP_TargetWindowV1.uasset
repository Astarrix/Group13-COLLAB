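; BP_TargetWindowV1 is a gameplay element representing a target window, acting as a container for a hand-placed set of window colliders.
; Its only custom logic, Return Window Colliders, hands callers a fixed array of those components, named in Box and W series.
; The event graph and construction script add no behavior, so any use of the colliders happens outside this Blueprint's graphs.
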(event EventBeginPlay
  (|CallParentFunction) ; This node is disabled and will not be called.\nDrag off pins to build functionality.
)

(event Collision|EventActorBeginOverlap
  (params (OtherActor :type Actor%20Object%20Reference)))

(event EventTick
  (params (DeltaSeconds :type Float%20%28single-precision%29)))

(fn ConstructionScript
  (|CallParentFunction))

(fn ReturnWindowColliders
  (return (Utilities|Array|MakeArray (Variables|Default|GetBox2) (Variables|Default|GetBox14) (Variables|Default|GetBox13) (Variables|Default|GetBox12) (Variables|Default|Getw) (Variables|Default|Getw5) (Variables|Default|Getw4) (Variables|Default|Getw1) (Variables|Default|Getw3) (Variables|Default|Getw2) (Variables|Default|GetBox11) (Variables|Default|GetBox7) (Variables|Default|GetBox6) (Variables|Default|GetBox5) (Variables|Default|GetBox4) (Variables|Default|GetBox8) (Variables|Default|GetBox3) (Variables|Default|GetBox9) (Variables|Default|GetBox10) (Variables|Default|GetBox1) (Variables|Default|GetBox15) (Variables|Default|Getw6) (Variables|Default|Getw21) (Variables|Default|Getw20) (Variables|Default|Getw22) (Variables|Default|Getw19) (Variables|Default|Getw18) (Variables|Default|Getw23) (Variables|Default|Getw24) (Variables|Default|Getw10) (Variables|Default|Getw9) (Variables|Default|Getw11) (Variables|Default|Getw8) (Variables|Default|Getw7) (Variables|Default|Getw17) (Variables|Default|Getw16) (Variables|Default|Getw15) (Variables|Default|Getw12) (Variables|Default|Getw14) (Variables|Default|Getw13))))