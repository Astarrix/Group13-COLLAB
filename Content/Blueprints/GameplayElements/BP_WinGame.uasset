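; BP_WinGame is a trigger actor that ends the game as a win when the player character overlaps its Box.
; On overlap it creates and shows the UIC_FinishReport widget, plays the Game_Win sound, shows the mouse cursor, switches to UI-only input and stops character movement.
; After a short delay it initializes the report with the player's BP_Character.
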(event OnComponentBeginOverlap(Box)
  (params (OverlappedComponent :type Primitive%20Component%20Object%20Reference) (OtherActor :type Actor%20Object%20Reference) (OtherComp :type Primitive%20Component%20Object%20Reference) (OtherBodyIndex :type Integer) (bFromSweep :type Boolean) (SweepResult :type Hit%20Result%20Structure%20%28by%20ref%29))
  (bind _returnvalue (Game|GetPlayerController 0))
  (bind _returnvalue_2 (Game|GetPlayerCharacter 0))
  (if (== OtherActor (Game|GetPlayerCharacter 0))
    (bind _returnvalue_3 (UserInterface|CreateWidget "/Game/UI/NewHUD/Panels/UIC_FinishReport.UIC_FinishReport_C" _returnvalue))
    (bind _output_get (Variables|Default|SetFinishReport _returnvalue_3))
    (bind _asbp_character (Utilities|Casting|CastToBP_Character _returnvalue_2))
    (UserInterface|Viewport|AddtoViewport _output_get 0)
    (Audio|PlaySound2D "/Game/Audio/SFXs/Music/Game_Win.Game_Win" 1.0 1.0 0.0 0 0)
    (Variables|/Script/Engine.PlayerController|SetbShowMouseCursor _returnvalue true)
    (Input|SetInputModeUIOnly _returnvalue 0 "DoNotLock" false)
    (Pawn|Components|CharacterMovement|SetMovementMode (Variables|/Script/Engine.Character|GetCharacterMovement _returnvalue_2) "MOVE_None" 0)
    (Utilities|FlowControl|Delay 1.0)
    (Default|Init _output_get _asbp_character)))

(fn ConstructionScript)