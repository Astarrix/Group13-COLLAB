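; BP_Area_Manager runs one level area's objectives: cleaning all its windows and destroying all its nests.
; It registers itself with both sets at BeginPlay and counts down as they report in.
; Activate highlights windows via custom depth, reveals splines and starts an area timer.
; Completion fires once, stopping the timer, notifying the game manager, opening the gate and moving the van, which NumPad 7 also triggers directly.
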(event Custom|Call%20Open%20Gate
  (bind _area_gate (Variables|Default|GetArea%20Gate))
  ;[1 1 1] Open Area gate
  (Utilities|IsValid _area_gate
    (:Is%20Valid
      (Default|OpenGate _area_gate))))

(event Custom|Area%20Completed
  ;[1 1 1] On area finished
  (Utilities|FlowControl|DoOnce false
    (:Completed
      (Utilities|Time|ClearandInvalidateTimerbyHandle (Variables|Default|GetArea%20Timer%20REF))
      (Default|IAreaCompleted (Variables|Default|GetGame%20Manager) self)
      (Development|PrintText (Utilities|Text|FormatText "Completed {name}" (Variables|Default|GetArea%20Name)) true true "(R=1.000000,G=0.419340,B=0.000000,A=1.000000)" 1e+01)
      (CallFunction|CallOpenGate)
      (CallFunction|MoveVan))))

(event Custom|Check%20Objectives
  ;[1 1 1] Check if Area Objectives met?
  (if (and (<= (Variables|Default|GetDirty%20windows) 0) (<= (Variables|Default|GetNests%20Remaining) 0))
    (CallFunction|AreaCompleted)))

(event Custom|Activate
  (for _array_element (Variables|Default|GetWindows)
    (Rendering|SetRenderCustomDepth (Variables|/Game/Blueprints/GameplayElements/Windows/BP_TargetWindowParent.BP_TargetWindowParent_C|GetStaticMesh _array_element) true))
  ;[1 1 1] Called when told to activate from game manager, starts area content
  (Utilities|FlowControl|DoOnce false
    (:Completed
      (bind _returnvalue (Utilities|Time|SetTimerbyEvent (delegate Custom|Area%20Timer) 1.0 true))
      (Variables|Default|SetArea%20Timer%20REF _returnvalue)
      (for _array_element_2 (Variables|Default|GetSpline)
        ;;[1 1 1] Make first spline in area NOT hidden
        (Rendering|SetActorHiddenInGame _array_element_2 false)))))

(event Custom|Area%20Timer
  ;[1 1 1] Called when told to activate from game manager, starts area content
  ;;[1 1 1] Area Timer
  (Math|Float|IncrementFloat (Variables|Default|GetArea%20Time)))

(event Custom|MoveVan
  ;[0 0.03342 1] MoveVan
  (Default|UpdateVanLocation (Variables|Default|GetNewVanLocation) (Variables|Default|GetVanTimeToNextLocation)))

(event EventBeginPlay
  (bind _windows (Variables|Default|GetWindows))
  (bind _nests (Variables|Default|GetNests))
  ;[1 1 1] Init chain, setting references
  ;;[1 1 1] Windows setup
  (if (!= (Utilities|Array|Length _windows) 0)
    (for _array_element _windows
      (Variables|/Game/Blueprints/GameplayElements/Windows/BP_TargetWindowParent.BP_TargetWindowParent_C|SetWindowManager _array_element self)))
  (bind _output_get (Variables|Default|SetTotal%20Number%20of%20windows (Utilities|Array|Length (Variables|Default|GetWindows))))
  (Variables|Default|SetDirty%20windows _output_get)
  (if (!= (Utilities|Array|Length _nests) 0)
    (for _array_element_2 _nests
      (Variables|/Game/Blueprints/GameplayElements/AI/bp_AiSpawner.bp_AiSpawner_C|SetArea%20Manager _array_element_2 self)))
  (bind _output_get_2 (Variables|Default|SetTotal%20Number%20of%20nests (Utilities|Array|Length (Variables|Default|GetNests))))
  (Variables|Default|SetNests%20Remaining _output_get_2))

(event EventIWindowCleaned
  ;[1 1 1] Update windows cleaned
  (bind _result (Math|Integer|DecrementInt (Variables|Default|GetDirty%20windows))
    (:%20%20
      (CallFunction|CheckObjectives)
      (if (<= _result 0)
        (CallFunction|MarkObjectiveasComplete "CleanWindows")
        (Development|PrintString "All windows cleaned!" true true "(R=0.000000,G=1.000000,B=0.937101,A=1.000000)" 5.0 "windowscleaned")
        (else
          (Development|PrintString (Utilities|String|ToString(Text) (Utilities|Text|FormatText "Window cleaned! Still {windows} windows remaining" _result)) true true "(R=0.000000,G=1.000000,B=0.937101,A=1.000000)" 5.0 "windowscleaned"))))))

(event EventINestDestroyed
  ;[1 1 1] Update nests destroyed
  (bind _result (Math|Integer|DecrementInt (Variables|Default|GetNests%20Remaining))
    (:%20%20
      (CallFunction|CheckObjectives)
      (if (<= _result 0)
        (Development|PrintString "All nests destroyed!" true true "(R=1.000000,G=0.000000,B=0.012286,A=1.000000)" 5.0 "nestsdestroyed")
        (else
          (Development|PrintString (Utilities|String|ToString(Text) (Utilities|Text|FormatText "Nest destroyed! Still {nests} nests remaining" _result)) true true "(R=1.000000,G=0.000000,B=0.012286,A=1.000000)" 5.0 "nestsdestroyed"))))))

(event Input|KeyboardEvents|NumPadSeven
  (params (Key :type Key%20Structure :default "None"))
  ;[0 0.03342 1] MoveVan
  (:Pressed
    (Default|UpdateVanLocation (Variables|Default|GetNewVanLocation) (Variables|Default|GetVanTimeToNextLocation))))

(fn ConstructionScript)