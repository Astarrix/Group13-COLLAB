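; Game manager that drives sequential progression through an ordered list of area managers.
; On BeginPlay it registers itself with each area and activates the first.
; When an area reports completion, it waits, shows the report card, opens that area's gate, moves the van and activates the next area.
; NumPad 7 also triggers the van move directly, and the all-areas-completed event is an empty stub.
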(event Custom|Open%20Gate
  ;[1 1 1] Call when you want to open the gate to the next area
  (Default|CallOpenGate (Variables|Default|GetCompleted%20Area%20REF)))

(event Custom|Activate%20Next%20Area
  (bind _area_managers (Variables|Default|GetArea%20Managers))
  ;[1 1 1] Call when you want to enable timers, and enemy spawns for the next area. (Will activate the area after the latest completed one)
  (if (>= (Variables|Default|GetAreas%20Competed) (Utilities|Array|Length _area_managers))
    (CallFunction|AllAreasCompleted)
    (else
      (Default|Activate (Utilities|Array|Get(acopy) _area_managers (Variables|Default|GetAreas%20Competed))))))

(event Custom|Move%20Van%20To%20Next%20Location
  (bind _area_managers (Variables|Default|GetArea%20Managers))
  (bind _areas_competed (Variables|Default|GetAreas%20Competed))
  (bind _returnvalue (- _areas_competed 1))
  (bind _output (Utilities|Array|Get(acopy) _area_managers _returnvalue))
  (bind _newvanlocation (Variables|/Game/Blueprints/GameplayElements/Manager/BP_Area_Manager.BP_Area_Manager_C|GetNewVanLocation _output))
  ;[1 1 1] Call when you want to move the van to the next location (not currently made!)
  (Default|UpdateVanLocation _newvanlocation (Variables|/Game/Blueprints/GameplayElements/Manager/BP_Area_Manager.BP_Area_Manager_C|GetVanTimeToNextLocation _output) (Transformation|GetActorTransform _newvanlocation)))

(event Custom|All%20areas%20completed
  ;[1 1 1] Gets called when all of the areas have been completed and active next area gets called
)

(event Custom|ShowReportCard
  (bind _reportref (Variables|Default|GetReportREF))
  ;[1 1 1] Call when you want the player to see the report for the completed area
  (Utilities|IsValid _reportref
    (:Is%20Valid
      (Default|ShowReport _reportref))))

(event EventBeginPlay
  ;[1 1 1] Init
  (for _array_element (Variables|Default|GetArea%20Managers)
    (Variables|/Game/Blueprints/GameplayElements/Manager/BP_Area_Manager.BP_Area_Manager_C|SetGame%20Manager _array_element self))
  (CallFunction|ActivateNextArea))

(event EventIAreaCompleted
  (params (Area%20Info :type BP%20Area%20Manager%20Object%20Reference))
  ;[1 1 1] Save reference to completed area, updates when new area completed
  (Variables|Default|SetCompleted%20Area%20REF Area%20Info)
  (Math|Integer|IncrementInt (Variables|Default|GetAreas%20Competed)
    (:%20%20
      (Utilities|FlowControl|Delay (Variables|Default|GetTime%20Until%20Area%20Completed%20Progression))
      (CallFunction|ShowReportCard)
      (CallFunction|OpenGate)
      (CallFunction|MoveVantoNextLocation)
      (CallFunction|ActivateNextArea))))

(event Input|KeyboardEvents|NumPadSeven
  (params (Key :type Key%20Structure :default "None"))
  (bind _area_managers (Variables|Default|GetArea%20Managers))
  (bind _areas_competed (Variables|Default|GetAreas%20Competed))
  (bind _returnvalue (- _areas_competed 1))
  (bind _output (Utilities|Array|Get(acopy) _area_managers _returnvalue))
  (bind _newvanlocation (Variables|/Game/Blueprints/GameplayElements/Manager/BP_Area_Manager.BP_Area_Manager_C|GetNewVanLocation _output))
  ;[1 1 1] Call when you want to move the van to the next location (not currently made!)
  (:Pressed
    (Default|UpdateVanLocation _newvanlocation (Variables|/Game/Blueprints/GameplayElements/Manager/BP_Area_Manager.BP_Area_Manager_C|GetVanTimeToNextLocation _output) (Transformation|GetActorTransform _newvanlocation))))

(fn ConstructionScript)