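; BP_Railgun is a railgun weapon Blueprint that hands its firing off to a line trace weapon reference.
; StartFire runs a validity check, then calls LineTraceFire on LineTraceWeaponRef, printing a debug string for either outcome.
; An unconnected leftover graph traces from the static mesh along the muzzle's forward vector and draws a debug beam, but never runs.
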(event EventStartFire
  (CallFunction|StartFire)
  (Utilities|IsValid 0
    (:Is%20Valid
      (Class|LineTraceWeapon|LineTraceFire (Variables|Default|GetLineTraceWeapon_Ref))
      (Development|PrintString "Firinggg"))
    (:Is%20Not%20Valid
      (Development|PrintString "Not Valid Mate" true true "(R=1.000000,G=0.000000,B=0.126577,A=1.000000)"))))

(fn ConstructionScript
  (|CallParentFunction))