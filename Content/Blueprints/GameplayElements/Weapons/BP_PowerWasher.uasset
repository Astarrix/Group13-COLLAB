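; Handheld power washer that toggles between soap and water spray, switching its Niagara effect and looping sound to match.
; While firing, a fast timer traces from the mouse cursor twice, alternating Visibility and Camera channels via FlipFlop, to aim the washer and foam ring.
; Target hits paint a render target and clean segments within the spray radius according to mode; other interface-implementing actors receive a wash message.
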(event Custom|Fire
  (if (Utilities|Enum|Equal(Enum) (Variables|/Game/Blueprints/Core/BP_PlayerController.BP_PlayerController_C|GetPlayerMovementState (.AsBP%20Player%20Controller (Utilities|Casting|CastToBP_PlayerController (Pawn|GetLocalViewingPlayerController (Variables|Default|GetOwning%20Character))))) "NewEnumerator1")
    (CallFunction|PowerWashTrace (Variables|Default|GetTo%20State))))

(event Custom|SwitchCleaningMode
  (params (ToState :type eWindowState%20Enum :default "NewEnumerator0"))
  (bind _returnvalue (Utilities|Enum|Equal(Enum) ToState "NewEnumerator1"))
  (Variables|Default|SetTo%20State ToState)
  (Effects|Components|ParticleSystem|SetBoolParameter (Variables|Default|GetNS_Spray) "isSoap" _returnvalue)
  (CallFunction|ChangeSound _returnvalue))

(event Custom|Start%20SFX
  ;[0.9424 0.2266 1] Start SFX
  (bind _returnvalue (Audio|SpawnSound2D (Variables|Default|GetCurrent%20Mode%20Sound) 1.0 1.0 0.0 0))
  (bind _output_get (Variables|Default|SetCurrent%20SFX _returnvalue))
  (Audio|Components|Audio|FadeIn _output_get 1.0 1.0 0.0 "Linear" :!class /Script/Engine.AudioComponent))

(event Custom|Stop%20SFX
  ;[0.9424 0.2266 1] Stop SFX
  (Audio|Components|Audio|FadeOut (Variables|Default|GetCurrent%20SFX) 1.0 0.0 "Linear" :!class /Script/Engine.AudioComponent))

(event Custom|Change%20Sound
  (params (isSoap :type Boolean))
  ;[0.9424 0.2266 1] Changes SFX based on soap or spray
  (if isSoap
    (Variables|Default|SetCurrent%20Mode%20Sound "/Game/Audio/SFXs/SoapGun_Spray.SoapGun_Spray")
    (else
      (Variables|Default|SetCurrent%20Mode%20Sound "/Game/Audio/SFXs/WaterGun_Spray.WaterGun_Spray"))))

(event Input|EnhancedActionEvents|EnhancedInputActionIA_SwitchMode
  (params (ActionValue :type Boolean) (ElapsedSeconds :type Float%20%28double-precision%29) (TriggeredSeconds :type Float%20%28double-precision%29) (InputAction :type Input%20Action%20Object%20Reference :default "/Game/Input/InputActions/IA_SwitchMode.IA_SwitchMode"))
  (:Started
    (bind _isa (Utilities|FlowControl|FlipFlop)
      (:A
        _)
      (:B
        _))
    (CallFunction|SwitchCleaningMode (select _isa "NewEnumerator2" "NewEnumerator1"))))

(event EventStartFire
  (bind _returnvalue (Utilities|Time|SetTimerbyEvent (EventDispatchers|CreateEvent :!event Custom|Fire) 0.01 true true))
  (Variables|Default|SetFireTimerHandle _returnvalue)
  (Components|Activation|SetActive (Variables|Default|GetNS_Spray) true false)
  (CallFunction|StartSFX))

(event EventStopFire
  (Utilities|Time|ClearandInvalidateTimerbyHandle (Variables|Default|GetFireTimerHandle))
  (Components|Activation|SetActive (Variables|Default|GetNS_Spray) false false)
  (CallFunction|StopSFX))

(event EventBeginPlay
  (CallFunction|SwitchCleaningMode "NewEnumerator1"))

(fn ConstructionScript
  (|CallParentFunction))

(fn PowerWashTrace
  (params (ToState :type eWindowState%20Enum :default "NewEnumerator0"))
  (bind _returnvalue (Game|GetPlayerController 0))
  (bind _sprayradius (Variables|Default|GetSprayRadius))
  (bind _ns_foamring (Variables|Default|GetNS_FoamRing))
  (bind (_worldlocation _worlddirection) (Game|Player|ConvertMouseLocationToWorldSpace _returnvalue))
  ;[0.01161 0.01161 0.01161] BP Magic that runs the thing twice with a diff parameter (to run both cam and vis)
  (Utilities|FlowControl|Sequence
    (:then_0
      _)
    (:then_1
      _))
  (bind _isa (Utilities|FlowControl|FlipFlop)
    (:A
      _)
    (:B
      _))
  (bind _outhit (Collision|LineTraceByChannel _worldlocation (+ _worldlocation (* _worlddirection (Math|Float|MakeLiteralFloat 3e+02))) (select _isa "TraceTypeQuery1" "TraceTypeQuery2") false (Utilities|Array|MakeArray self (Variables|Default|GetOwning%20Character)) "ForOneFrame"))
  (Transformation|SetActorRotation (Math|Rotator|FindLookatRotation (Transformation|GetActorLocation) (.ImpactPoint (Collision|BreakHitResult _outhit))))
  (Transformation|SetWorldLocation _ns_foamring (.ImpactPoint (Collision|BreakHitResult _outhit)) false false)
  (Transformation|SetRelativeRotation _ns_foamring (Math|Rotator|MakeRotator (.Roll (Math|Rotator|BreakRotator (Math|Conversions|RotationFromXVector (.Normal (Collision|BreakHitResult _outhit))))) (+ (.Pitch (Math|Rotator|BreakRotator (Math|Conversions|RotationFromXVector (.Normal (Collision|BreakHitResult _outhit))))) 9e+01) (.Yaw (Math|Rotator|BreakRotator (Math|Conversions|RotationFromXVector (.Normal (Collision|BreakHitResult _outhit)))))) false false)
  (bind _asa_target (Utilities|Casting|CastToA_Target (.HitActor (Collision|BreakHitResult _outhit)))
    (:then
      (Default|DrawtoRenderTarget _asa_target (.ImpactPoint (Collision|BreakHitResult _outhit)) _sprayradius)
      (bind _outhits (Collision|MultiSphereTraceByChannel (.ImpactPoint (Collision|BreakHitResult _outhit)) (.ImpactPoint (Collision|BreakHitResult _outhit)) _sprayradius "TraceTypeQuery1" false 0 "ForOneFrame"))
      (for _array_element _outhits
        (if (== (.HitActor (Collision|BreakHitResult _array_element)) _asa_target)
          (Default|CleanWindowSegment _asa_target (.HitComponent (Collision|BreakHitResult _array_element)) ToState))))
    (:CastFailed
      (if (Utilities|DoesObjectImplementInterface (.HitActor (Collision|BreakHitResult _outhit)) "/Game/Tools/BPI_ActorCalls.BPI_ActorCalls_C")
        (Class|BPIActorCalls|AttemptWash(Message) (.HitActor (Collision|BreakHitResult _outhit)))))))