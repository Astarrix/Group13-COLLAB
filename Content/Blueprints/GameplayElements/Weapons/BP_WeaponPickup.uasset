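; Weapon pickup that hands a projectile weapon to an actor colliding with it, if that actor can take one.
; CanBePickedUp asks the colliding actor through the BPI_ActorCalls interface whether it accepts a weapon, and gets its character reference.
; On approval, ObjectPickedUp spawns a BP_Weapon_Projectile at the pickup's transform, passes that character to its PickedUp function, and returns whether the pickup succeeded.
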(fn ConstructionScript)

(fn ObjectPickedUp
  (params (CollidingActor :type Actor%20Object%20Reference))
  (bind (_canbepickedup _character_reference) (CallFunction|CanbePickedUp CollidingActor))
  (if _canbepickedup
    (bind _returnvalue (Game|SpawnActorfromClass "/Game/Blueprints/GameplayElements/Weapons/BP_Weapon_Projectile.BP_Weapon_Projectile_C" (Transformation|GetActorTransform) "AdjustIfPossibleButAlwaysSpawn" "MultiplyWithRoot" 0 0))
    (Default|PickedUp _returnvalue _character_reference)
    (return true)
    (else
      (return false))))

(fn CanbePickedUp
  (params (CollidingActor :type Actor%20Object%20Reference))
  (if (Utilities|DoesObjectImplementInterface CollidingActor "/Game/Tools/BPI_ActorCalls.BPI_ActorCalls_C")
    (bind (_canpickupweapon _character_reference) (Class|BPIActorCalls|AttemptPickUpWeapon(Message) CollidingActor))
    (return _canpickupweapon _character_reference)
    (else
      (return false 0))))