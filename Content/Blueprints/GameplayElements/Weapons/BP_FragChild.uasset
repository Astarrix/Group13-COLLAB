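; BP_FragChild is a timed frag grenade actor that explodes after a BounceDelay set off at BeginPlay.
; The explosion applies radial damage, fires a RadialForce impulse on physics props, plays sound and a Niagara effect, shakes player 0's camera, then destroys the actor.
; Mesh hits play a floor-bounce sound, placed at world origin rather than at the impact point.
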(event OnComponentHit(StaticMesh)
  (params (HitComponent :type Primitive%20Component%20Object%20Reference) (OtherActor :type Actor%20Object%20Reference) (OtherComp :type Primitive%20Component%20Object%20Reference) (NormalImpulse :type Vector :default "0, 0, 0") (Hit :type Hit%20Result%20Structure%20%28by%20ref%29))
  (Audio|PlaySoundatLocation "/Game/Audio/SFXs/GrenadeHitFloor.GrenadeHitFloor" "0, 0, 0" "0, 0, 0" 1.0 1.0 0.0 0 0 0 0))

(event EventBeginPlay
  (bind _staticmesh (Variables|Default|GetStaticMesh))
  (bind _returnvalue (Transformation|GetWorldLocation _staticmesh))
  (Utilities|FlowControl|Delay (Variables|Default|GetBounce%20Delay))
  (Game|Damage|ApplyRadialDamage (Variables|Default|GetBase%20Damage) (Transformation|GetActorLocation self) (Variables|Default|GetDamage%20Radius) 0 0 self 0 false "ECC_Visibility")
  ;[0.2396 0.479 1] Physics for Environment Props
  (Class|RadialForceComponent|FireImpulse (Variables|Default|GetRadialForce))
  (Audio|PlaySoundatLocation "/Game/Audio/SFXs/grenade-explosion-14-190266.grenade-explosion-14-190266" _returnvalue "0, 0, 0" 1.0 1.0 0.0 0 0 0 0)
  ;[0.05725 1 0] Explosion Effect
  (Niagara|SpawnSystematLocation "/Game/VFX/NS_Explosion.NS_Explosion" _returnvalue)
  ;[0.07438 1 0] Camera Shake
  (CallFunction|CameraShakewithOptions (Game|GetPlayerCameraManager 0) true 2 1)
  (Actor|DestroyActor self))

(fn ConstructionScript)