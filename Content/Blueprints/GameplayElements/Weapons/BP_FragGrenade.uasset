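; BP_FragGrenade is a throwable frag grenade weapon that spawns a projectile when fired.
; StartFire checks the frag count and a cooldown flag, plays a pin-pull sound at world origin, then waits before spawning at the MuzzlePoint transform.
; Each throw decrements the count, either resetting the cooldown after a delay or, once empty, destroying the actor and calling RemoveAllWidgets.
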(event EventStartFire
  (bind _muzzlepoint (Variables|Default|GetMuzzlePoint))
  ;[1 1 1] Checking for Ammo
  (if (<= (Variables|Default|GetCurrentFrag) (Variables|Default|GetMaxFrags))
    ;[0.06435 1 0] Throw Delay
    (if (Variables|Default|GetThrowDelayFinished)
      (Variables|Default|SetThrowDelayFinished false)
      ;[0.1042 1 0] Play SFX
      (Audio|PlaySoundatLocation "/Game/Audio/SFXs/GrenadePinPulled.GrenadePinPulled" "0, 0, 0" "0, 0, 0" 1.0 1.0 0.0 0 0 0 0)
      (Utilities|FlowControl|Delay (Variables|Default|GetPinPullDelay))
      (Game|SpawnActorfromClass "/Game/Blueprints/GameplayElements/Weapons/BP_FragChild.BP_FragChild_C" (Math|Transform|MakeTransform (Transformation|GetWorldLocation _muzzlepoint) (Transformation|GetWorldRotation _muzzlepoint)) "Undefined" "MultiplyWithRoot" 0 0)
      ;[0.08761 1 0] Decrement Ammo
      (Math|Integer|DecrementInt (Variables|Default|GetCurrentFrag)
        (:%20%20
          (if (<= (Variables|Default|GetCurrentFrag) (Variables|Default|GetFragsEmpty))
            (Actor|DestroyActor self)
            (Viewport|RemoveAllWidgets)
            (else
              ;[0.05007 1 0] Fire Delay
              (Utilities|FlowControl|Delay (Variables|Default|GetThrowDelayTime))
              (Variables|Default|SetThrowDelayFinished true))))))))

(fn ConstructionScript
  (|CallParentFunction))