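; BP_WaterJet_Gun is a water jet weapon that attaches to the owning character's right arm mount and enables player input when picked up.
; Starting IA_Shoot fires one debug-drawn visibility line trace forward from the muzzle, while holding it only prints a message.
; Releasing or canceling the input calls StopFire.
; The gun is unfinished: the trace result is unused, a BP_FloorAI hit cast is unconnected, and Dropped is empty.
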(event Custom|PickedUp
  (params (OwningCharacter :type BP%20Character%20Object%20Reference))
  (Transformation|AttachComponentToComponent (Variables|/Game/Blueprints/Core/BP_Character.BP_Character_C|GetRightArmMount OwningCharacter) "None" "SnapToTarget" "SnapToTarget" "KeepRelative" true)
  (Input|EnableInput (Game|GetPlayerController 0)))

(event Custom|Dropped)

(event Input|EnhancedActionEvents|EnhancedInputActionIA_Shoot
  (params (ActionValue :type Vector%202D%20Structure) (ElapsedSeconds :type Float%20%28double-precision%29) (TriggeredSeconds :type Float%20%28double-precision%29) (InputAction :type Input%20Action%20Object%20Reference :default "/Game/Input/InputActions/IA_Shoot.IA_Shoot"))
  (:Triggered
    (Development|PrintString "I am water gunning"))
  (:Started
    (bind _outhit (Collision|LineTraceByChannel (Transformation|GetWorldLocation (Variables|Default|Get_Muzzle)) (+ (* (Math|Vector|GetForwardVector (Variables|Default|Get_Muzzle)) (Variables|Default|GetRayDistance)) (Transformation|GetWorldLocation (Variables|Default|Get_Muzzle))) "TraceTypeQuery1" false 0 "ForDuration")))
  (:Canceled
    (Class|WeaponBase|StopFire :!label _label))
  (:Completed
    (goto _label)))

(fn ConstructionScript)