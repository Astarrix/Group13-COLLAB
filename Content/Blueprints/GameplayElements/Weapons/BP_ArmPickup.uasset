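; BP_ArmPickup is a world pickup that grants a character a left or right arm weapon of a configured ArmType.
; Its construction script shows the arm class's default mesh on the pickup.
; On pickup, it asks the colliding actor through BPI_ActorCalls whether it can take that arm side.
; If so, it spawns the arm at the pickup's transform and initializes it with the owning character and side.
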(fn ConstructionScript
  (Components|StaticMesh|SetStaticMesh (Variables|Default|GetPickupMesh) (.ArmMesh (Utilities|GetClassDefaults (Variables|Default|GetArmType)))))

(fn ObjectPickedUp
  (params (CollidingActor :type Actor%20Object%20Reference))
  (bind (_canbepickedup _character_reference) (CallFunction|CanbePickedUp CollidingActor))
  (if _canbepickedup
    (bind _returnvalue (Game|SpawnActorfromClass (Variables|Default|GetArmType) (Transformation|GetActorTransform) "AdjustIfPossibleButAlwaysSpawn" "MultiplyWithRoot" 0 0))
    (Default|Init _returnvalue _character_reference (Variables|Default|GetisLeftArm))
    (return true)
    (else
      (return false))))

(fn CanbePickedUp
  (params (CollidingActor :type Actor%20Object%20Reference))
  (if (Utilities|DoesObjectImplementInterface CollidingActor "/Game/Tools/BPI_ActorCalls.BPI_ActorCalls_C")
    (bind (_canpickupweapon _character_reference) (Class|BPIActorCalls|AttemptPickUpWeapon(Message) CollidingActor (Variables|Default|GetisLeftArm)))
    (return _canpickupweapon _character_reference)
    (else
      (return false 0))))