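; BP_ArmParent is the base Blueprint for left or right arm weapons that attach to a character and can be dropped.
; Init attaches the arm to the matching mount and enables player input, so side-specific actions call StartFire and StopFire, both empty here.
; Drop spawns a BP_ArmPickup carrying the side and class, notifies the owning character, then destroys the arm.
; The construction script applies the configurable arm mesh.
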(event Custom|StartFire)

(event Custom|StopFire)

(event Custom|Drop
  (Input|DisableInput (Game|GetPlayerController 0))
  (Game|SpawnActorfromClass "/Game/Blueprints/GameplayElements/Weapons/BP_ArmPickup.BP_ArmPickup_C" (Transformation|GetActorTransform) "Undefined" "MultiplyWithRoot" 0 (Variables|Default|GetIs%20Left%20Arm) (Utilities|GetClass self) 0)
  (Default|SetDropArmState (Variables|Default|GetOwning%20Character) (Variables|Default|GetIs%20Left%20Arm))
  (Actor|DestroyActor))

(event Custom|Init
  (params (OwningCharacter :type BP%20Character%20Object%20Reference) (IsLeftArm :type Boolean))
  (bind _output_get (Variables|Default|SetOwning%20Character OwningCharacter))
  (CallFunction|ManageAttachment true IsLeftArm _output_get)
  (Input|EnableInput (Game|GetPlayerController 0)))

(event Custom|ManageAttachment
  (params (IsAttaching :type Boolean) (IsLeftArm :type Boolean) (AttachedCharacter :type BP%20Character%20Object%20Reference))
  (Variables|Default|SetIs%20Left%20Arm IsLeftArm)
  (if IsAttaching
    (Transformation|AttachComponentToComponent (.AsScene%20Component (Utilities|Casting|CastToSceneComponent (Utilities|SelectObject (Variables|/Game/Blueprints/Core/BP_Character.BP_Character_C|GetLeftArmMount AttachedCharacter) (Variables|/Game/Blueprints/Core/BP_Character.BP_Character_C|GetRightArmMount AttachedCharacter) IsLeftArm))) "None" "SnapToTarget" "SnapToTarget" "KeepRelative" false)
    (else
      (Transformation|DetachFromActor "KeepWorld" "KeepWorld" "KeepWorld"))))

(event Input|EnhancedActionEvents|EnhancedInputActionIA_RightArmActivate
  (params (ActionValue :type Vector%202D%20Structure) (ElapsedSeconds :type Float%20%28double-precision%29) (TriggeredSeconds :type Float%20%28double-precision%29) (InputAction :type Input%20Action%20Object%20Reference :default "/Game/Input/InputActions/IA_RightArmActivate.IA_RightArmActivate"))
  (:Started
    (if (not (Variables|Default|GetIs%20Left%20Arm))
      (CallFunction|StartFire)))
  (:Canceled
    (if (not (Variables|Default|GetIs%20Left%20Arm)) :!label _label
      (CallFunction|StopFire)))
  (:Completed
    (goto _label)))

(event Input|EnhancedActionEvents|EnhancedInputActionIA_Drop
  (params (ActionValue :type Boolean) (ElapsedSeconds :type Float%20%28double-precision%29) (TriggeredSeconds :type Float%20%28double-precision%29) (InputAction :type Input%20Action%20Object%20Reference :default "/Game/Input/InputActions/IA_Drop.IA_Drop"))
  (:Started
    (CallFunction|Drop)))

(event Input|EnhancedActionEvents|EnhancedInputActionIA_LeftArmActivate
  (params (ActionValue :type Boolean) (ElapsedSeconds :type Float%20%28double-precision%29) (TriggeredSeconds :type Float%20%28double-precision%29) (InputAction :type Input%20Action%20Object%20Reference :default "/Game/Input/InputActions/IA_LeftArmActivate.IA_LeftArmActivate"))
  (:Started
    (if (Variables|Default|GetIs%20Left%20Arm)
      (CallFunction|StartFire)))
  (:Canceled
    (if (Variables|Default|GetIs%20Left%20Arm) :!label _label
      (CallFunction|StopFire)))
  (:Completed
    (goto _label)))

(fn ConstructionScript
  (Components|StaticMesh|SetStaticMesh (Variables|Default|GetStaticMesh) (Variables|Default|GetArmMesh)))