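; Grenade launcher projectile that explodes as soon as its static mesh registers a hit.
; The hit applies full radial damage at the actor's location and fires a radial force impulse to blast environment props.
; It then plays an explosion sound and Niagara effect, shakes the first player's camera with an FOV shake, and destroys itself.
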(event OnComponentHit(StaticMesh)
  (params (HitComponent :type Primitive%20Component%20Object%20Reference) (OtherActor :type Actor%20Object%20Reference) (OtherComp :type Primitive%20Component%20Object%20Reference) (NormalImpulse :type Vector :default "0, 0, 0") (Hit :type Hit%20Result%20Structure%20%28by%20ref%29))
  (bind _staticmesh (Variables|Default|GetStaticMesh))
  (bind _returnvalue (Transformation|GetWorldLocation _staticmesh))
  (Game|Damage|ApplyRadialDamage (Variables|Default|GetBase%20Damage) (Transformation|GetActorLocation self) (Variables|Default|GetDamage%20Radius) 0 0 self 0 true "ECC_Visibility")
  ;[0.07232 0.2602 0.4375] Blasts the Environment Props
  (Class|RadialForceComponent|FireImpulse (Variables|Default|GetRadialForce))
  ;[0.07221 0.5536 1] SFX and VFX
  (Audio|PlaySoundatLocation "/Game/Audio/SFXs/grenade-explosion-14-190266.grenade-explosion-14-190266" _returnvalue "0, 0, 0" 1.0 1.0 0.0 0 0 0 0)
  (Niagara|SpawnSystematLocation "/Game/VFX/NS_Explosion.NS_Explosion" _returnvalue)
  ;[0 0.6145 1] Camera Shake
  (CallFunction|CameraShakewithOptions (Game|GetPlayerCameraManager 0) true 2 1)
  (Actor|DestroyActor))

(fn ConstructionScript)