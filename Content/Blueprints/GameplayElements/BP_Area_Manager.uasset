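; BP_Area_Manager tracks an area's cleaning and combat objectives, dirty windows and nests, and opens the AreaGate when both are done.
; On BeginPlay it registers itself as each window's WindowManager and counts the windows.
; Window-cleaned and nest-destroyed events decrement counters, check completion and print progress on screen.
; The nest-count setup is unconnected, so NestsRemaining is never initialised in the graph.
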(event Custom|Area%20Completed
  ;[1 1 1] On area finished
  (Default|OpenGate (Variables|Default|GetArea%20Gate)))

(event Custom|Check%20Objectives
  ;[1 1 1] Check if Area Objectives met?
  (if (and (<= (Variables|Default|GetDirty%20windows) 0) (<= (Variables|Default|GetNests%20Remaining) 0))
    (CallFunction|AreaCompleted)))

(event EventBeginPlay
  (bind _windows (Variables|Default|GetWindows))
  ;[1 1 1] Init chain, setting references
  ;;[1 1 1] Windows setup
  (if (!= (Utilities|Array|Length _windows) 0)
    (for _array_element _windows
      (Variables|/Game/Blueprints/GameplayElements/BP_TargetWindowParent.BP_TargetWindowParent_C|SetWindowManager _array_element self)))
  (bind _output_get (Variables|Default|SetTotal%20Number%20of%20windows (Utilities|Array|Length (Variables|Default|GetWindows))))
  (Variables|Default|SetDirty%20windows _output_get))

(event EventIWindowCleaned
  ;[1 1 1] Update windows cleaned
  (bind _result (Math|Integer|DecrementInt (Variables|Default|GetDirty%20windows))
    (:%20%20
      (CallFunction|CheckObjectives)
      (if (<= _result 0)
        (Development|PrintString "All windows cleaned!" true true "(R=0.000000,G=1.000000,B=0.937101,A=1.000000)" 5.0 "windowscleaned")
        (else
          (Development|PrintString (Utilities|String|ToString(Text) (Utilities|Text|FormatText "Window cleaned! Still {windows} windows remaining" _result)) true true "(R=0.000000,G=1.000000,B=0.937101,A=1.000000)" 5.0 "windowscleaned"))))))

(event EventINestDestroyed
  ;[1 1 1] Update nests destroyed
  (bind _result (Math|Integer|DecrementInt (Variables|Default|GetNests%20Remaining))
    (:%20%20
      (CallFunction|CheckObjectives)
      (if (<= _result 0)
        (Development|PrintString "All nests destroyed!" true true "(R=1.000000,G=0.000000,B=0.012286,A=1.000000)" 5.0 "nestsdestroyed")
        (else
          (Development|PrintString (Utilities|String|ToString(Text) (Utilities|Text|FormatText "Nest destroyed! Still {nests} nests remaining" _result)) true true "(R=1.000000,G=0.000000,B=0.012286,A=1.000000)" 5.0 "nestsdestroyed"))))))

(fn ConstructionScript)