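; Parent Blueprint for washable windows that players clean segment by segment, notifying the WindowManager when all are done.
; At startup it captures a UV-unwrap render target, letting a brush material paint world-space hits into a second target used as the opacity mask.
; Colliders supplied through ReturnWindowColliders, empty here, advance through three ordered wash states.
; Completing all segments flashes the materials, swaps to a clean material and plays a sound.
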(event Custom|CleanWindowSegment
  (params (HitComponent :type Primitive%20Component%20Object%20Reference) (ToState :type eWindowState%20Enum :default "NewEnumerator0"))
  (bind _segmentstate (Variables|Default|GetSegmentState))
  (bind (_value _returnvalue) (Utilities|Map|Find _segmentstate HitComponent))
  (if _returnvalue
    (if (and (Utilities|Enum|Equal(Enum) _value "NewEnumerator0") (Utilities|Enum|Equal(Enum) ToState "NewEnumerator1"))
      (Utilities|Map|Add _segmentstate HitComponent "NewEnumerator1")
      (elif (and (Utilities|Enum|Equal(Enum) _value "NewEnumerator1") (Utilities|Enum|Equal(Enum) ToState "NewEnumerator2"))
        (Utilities|Map|Add _segmentstate HitComponent "NewEnumerator2") ; ToClean
        (Collision|SetCollisionResponsetoChannel HitComponent "ECC_Visibility" "ECR_Overlap")
        (if (CallFunction|CheckAllWindowStates)
          (CallFunction|WindowCleaned)
          (else
            (Transformation|DetachFromComponent HitComponent "KeepRelative" "KeepRelative" "KeepRelative" true)
            (Components|DestroyComponent HitComponent)))))))

(event Custom|InitWashState
  (bind _colliders (CallFunction|ReturnWindowColliders))
  (for _array_element _colliders
    (Utilities|Map|Add (Variables|Default|GetSegmentState) _array_element "NewEnumerator0")))

(event Custom|WindowCleaned
  (Utilities|FlowControl|DoOnce false
    (:Completed
      (bind _flashvalue (Timeline|FlashMaterial PlayFromStart)
        (:Update
          (for _array_element (Variables|Default|GetMaterialInstances)
            (Rendering|Material|SetScalarParameterValue _array_element "FlashValue" _flashvalue :!class /Script/Engine.MaterialInstanceDynamic)
            ;[1 1 1] Changes mat to clean after completion.
            (Utilities|FlowControl|Delay 0.2)
            (Rendering|Material|SetMaterial (Variables|Default|GetStaticMesh) 0 "/Game/Blueprints/PowerWashing/Materials/M_CleanWindow.M_CleanWindow")
            (Utilities|FlowControl|DoOnce false
              (:Completed
                (Default|CallOnWindowCleaned)
                (Audio|PlaySoundatLocation "/Game/Audio/SFXs/Window_Cleaned.Window_Cleaned" (Transformation|GetActorLocation) "0, 0, 0" 1.0 1.0 0.0 0 0 0 0)
                ;[1 1 1] Call interface - window cleaned
                (Utilities|FlowControl|DoOnce false
                  (:Completed
                    (Class|BPIAreaTracking|IWindowCleaned(Message) (Variables|Default|GetWindowManager))))))))))))

(event EventBeginPlay
  ;[1 1 1] Put Material Instance in array and create render targets.
  (Utilities|FlowControl|Delay 0.2)
  (CallFunction|InitWashState)
  (for _index (range 0 (- (Rendering|Material|GetNumMaterials (Variables|Default|GetStaticMesh)) 1))
    (bind _returnvalue (Rendering|Material|CreateDynamicMaterialInstance (Variables|Default|GetStaticMesh) _index (Variables|Default|GetSource%20Material) "None" :!class /Script/Engine.PrimitiveComponent))
    (Utilities|Array|Add (Variables|Default|GetMaterialInstances) _returnvalue))
  (Utilities|FlowControl|Sequence
    (:then_0
      (bind _returnvalue_2 (Rendering|CreateRenderTarget2D 1024 1024 "RTF_RGBA16f"))
      (bind _output_get (Variables|Default|SetRt_Unwrap _returnvalue_2))
      (Variables|/Script/Engine.SceneCaptureComponent2D|SetTextureTarget (Variables|Default|GetSceneCaptureComponent2D) _output_get)
      (Rendering|SceneCapture|ShowOnlyActorComponents (Variables|Default|GetSceneCaptureComponent2D) self false))
    (:then_1
      (bind _returnvalue_3 (Rendering|CreateRenderTarget2D 1024 1024 "RTF_RGBA16f"))
      (Variables|Default|SetRT_Hit _returnvalue_3)
      (for _array_element (Variables|Default|GetMaterialInstances)
        (Class|MaterialInstanceDynamic|SetTextureParameterValuebyInfo _array_element (Utilities|Struct|MakeMaterialParameterInfo "Opacity Mask" "BlendParameter" 0) (Variables|Default|GetRT_Hit)))
      (Rendering|ClearRenderTarget2D (Variables|Default|GetRT_Hit)))
    (:then_2
      ;[1 1 1] Capture UV Unwrap and then reset texure to normal
      (Transformation|SetWorldRotation (Variables|Default|GetSceneCaptureComponent2D) "-90.000000,-90.000000,0.000000" false false)
      (for _index_2 (range 0 (- (Rendering|Material|GetNumMaterials (Variables|Default|GetStaticMesh)) 1))
        (Rendering|Material|SetMaterial (Variables|Default|GetStaticMesh) _index_2 "/Game/Blueprints/PowerWashing/Materials/M_Unwrap.M_Unwrap"))
      (Rendering|SceneCapture|CaptureScene (Variables|Default|GetSceneCaptureComponent2D) :!class /Script/Engine.SceneCaptureComponent2D)
      (for (_array_element_2 _array_index) (Variables|Default|GetMaterialInstances)
        (Rendering|Material|SetMaterial (Variables|Default|GetStaticMesh) _array_index _array_element_2))
      (bind _returnvalue_4 (Rendering|Material|CreateDynamicMaterialInstance "/Game/Blueprints/PowerWashing/Materials/M_Brush.M_Brush" "None" "None" :!class /Script/Engine.KismetMaterialLibrary))
      (bind _output_get_2 (Variables|Default|SetMI_Brush _returnvalue_4))
      (Rendering|Material|SetTextureParameterValue _output_get_2 "Unwrapped" (Variables|Default|GetRt_Unwrap)))))

(fn ConstructionScript
  (Components|StaticMesh|SetStaticMesh (Variables|Default|GetStaticMesh) (Variables|Default|GetSource%20Mesh)))

(fn DrawtoRenderTarget
  (params (Impact%20Point :type Vector) (Brush%20Size :type Float%20%28double-precision%29))
  (Rendering|Material|SetScalarParameterValue (Variables|Default|GetMI_Brush) "Size" Brush%20Size :!class /Script/Engine.MaterialInstanceDynamic)
  (Rendering|Material|SetVectorParameterValue (Variables|Default|GetMI_Brush) "Position" (Math|Conversions|ToLinearColor(Vector) Impact%20Point) :!class /Script/Engine.MaterialInstanceDynamic)
  (Rendering|DrawMaterialtoRenderTarget (Variables|Default|GetRT_Hit) (Variables|Default|GetMI_Brush)))

(fn ModifyBrushSize
  (params (BrushSize :type Float%20%28double-precision%29))
  (Rendering|Material|SetScalarParameterValue (Variables|Default|GetMI_Brush) "Size" BrushSize :!class /Script/Engine.MaterialInstanceDynamic))

(fn CheckAllWindowStates
  (bind _segmentstate (Variables|Default|GetSegmentState))
  (bind _keys (Utilities|Map|Keys _segmentstate))
  (for _array_element _keys
    (if (or (Utilities|Enum|Equal(Enum) (.Value (Utilities|Map|Find _segmentstate _array_element)) "NewEnumerator0") (Utilities|Enum|Equal(Enum) (.Value (Utilities|Map|Find _segmentstate _array_element)) "NewEnumerator1"))
      (LocalVariables|SetLOCAL_isAllCleaned false)))
  (return (LocalVariables|GetLOCAL_isAllCleaned)))

(fn ReturnWindowColliders
  (return 0))