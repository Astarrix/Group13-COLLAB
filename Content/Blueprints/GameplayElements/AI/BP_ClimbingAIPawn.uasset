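; Climbing bug enemy pawn that hands surface pathfinding and body rotation to a plugin SpiderAIController.
; On begin play or bug spawn it sets the controller's move speed and starts pathfinding.
; A stopping-distance overlap halts it near the player, while Tick turns a separate arrow toward the player to aim its shots.
; On death it spawns an effect, unpossesses the controller and calls PawnDead.
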(event OnComponentBeginOverlap(_StoppingDistance)
  (params (OverlappedComponent :type Primitive%20Component%20Object%20Reference) (OtherActor :type Actor%20Object%20Reference) (OtherComp :type Primitive%20Component%20Object%20Reference) (OtherBodyIndex :type Integer) (bFromSweep :type Boolean) (SweepResult :type Hit%20Result%20Structure%20%28by%20ref%29))
  ;[0.4745 1 0.4745] Stops moving when close to player
  (if (Actor|ActorHasTag OtherActor "Player")
    (Variables|/SpiderNavigation/SpiderAIController.SpiderAIController_C|SetMoveSpeed (Variables|Default|GetSpiderAIController) 0.0)))

(event OnComponentEndOverlap(_StoppingDistance)
  (params (OverlappedComponent :type Primitive%20Component%20Object%20Reference) (OtherActor :type Actor%20Object%20Reference) (OtherComp :type Primitive%20Component%20Object%20Reference) (OtherBodyIndex :type Integer))
  ;[0.4745 1 0.4745] Starts moving again when no longer overlapping with player
  (if (Actor|ActorHasTag OtherActor "Player")
    (Variables|/SpiderNavigation/SpiderAIController.SpiderAIController_C|SetMoveSpeed (Variables|Default|GetSpiderAIController) (Variables|Default|GetBaseSpeed))))

(event EventHandleHealthDead
  (params (causer :type Controller%20Object%20Reference))
  (Niagara|SpawnSystematLocation 0 (Transformation|GetActorLocation))
  (Pawn|UnPossess (Pawn|GetController))
  (Class|AIPawn|PawnDead))

(event EventBugSpawned
  ;[0.4745 1 0.4745] Sets the controller and then calls the function from the plugin to start the pathfinding
  (bind _asspider_aicontroller (Utilities|Casting|CastToSpiderAIController (Pawn|GetController)))
  (bind _output_get (Variables|Default|SetSpiderAIController _asspider_aicontroller))
  (Variables|/SpiderNavigation/SpiderAIController.SpiderAIController_C|SetMoveSpeed _output_get (Variables|Default|GetBaseSpeed))
  (Default|PawnSpawned _asspider_aicontroller))

(event EventBeginPlay
  ;[0.4745 1 0.4745] Sets the controller and then calls the function from the plugin to start the pathfinding
  (bind _asspider_aicontroller (Utilities|Casting|CastToSpiderAIController (Pawn|GetController)))
  (bind _output_get (Variables|Default|SetSpiderAIController _asspider_aicontroller))
  (Variables|/SpiderNavigation/SpiderAIController.SpiderAIController_C|SetMoveSpeed _output_get (Variables|Default|GetBaseSpeed))
  (Default|PawnSpawned _asspider_aicontroller))

(event EventTick
  (params (DeltaSeconds :type Float%20%28single-precision%29))
  (bind _returnvalue (Transformation|GetActorLocation))
  (bind _returnvalue_2 (Game|GetPlayerCharacter 0))
  (bind _asbp_character (Utilities|Casting|CastToBP_Character _returnvalue_2))
  (bind _returnvalue_3 (Transformation|GetActorLocation _asbp_character))
  (bind _returnvalue_4 (Math|Rotator|FindLookatRotation _returnvalue _returnvalue_3))
  ;[0.4745 1 0.4745] Rotates the direction the bug shoots in since the bug irotation is controlled in the contoller.
  (Transformation|SetWorldRotation (Variables|Default|Get_FacePlayerArrow) (Math|Rotator|MakeRotator (.roll _returnvalue_4) (.pitch _returnvalue_4) (.yaw _returnvalue_4)) false false))

(event EventControlRotation
  (params (Player :type Actor%20Object%20Reference))
  ;[0.4745 1 0.4745] Rotates the direction the bug shoots in since the bug irotation is controlled in the contoller.
)

(event EventHandleHealthDamaged
  (params (current :type Float%20%28single-precision%29) (max :type Float%20%28single-precision%29) (change :type Float%20%28single-precision%29)))

(fn ConstructionScript)