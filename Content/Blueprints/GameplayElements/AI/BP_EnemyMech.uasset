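; BP_EnemyMech is an enemy mech Blueprint that keeps its left and right arrow components aimed at the player.
; BeginPlay caches the player as BP_Character.
; Each Tick rotates both arrows with look-at rotations toward a point slightly below the center of the player's actor bounds.
; The arrow-control and health-damage events are empty stubs, and no firing logic is present.
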(event Custom|ControlArrowRotation_1)

(event Custom|Handle_HealthDamaged_1
  (params (current :type Float%20%28single-precision%29) (max :type Float%20%28single-precision%29) (change :type Float%20%28single-precision%29)))

(event EventTick
  (params (DeltaSeconds :type Float%20%28single-precision%29))
  (bind __leftarrow (Variables|Default|Get_LeftArrow))
  (bind __righttarrow (Variables|Default|Get_RighttArrow))
  (Utilities|FlowControl|Sequence
    (:then_0
      (Transformation|SetWorldRotation __leftarrow (Math|Rotator|MakeRotator (.roll (Math|Rotator|FindLookatRotation (Transformation|GetWorldLocation __leftarrow) (Math|Vector|MakeVector (.x (.Origin (Collision|GetActorBounds (stale EventBeginPlay _output_get) false false))) (.y (.Origin (Collision|GetActorBounds (stale EventBeginPlay _output_get) false false))) (- (.z (.Origin (Collision|GetActorBounds (stale EventBeginPlay _output_get) false false))) 1e+02)))) (.pitch (Math|Rotator|FindLookatRotation (Transformation|GetWorldLocation __leftarrow) (Math|Vector|MakeVector (.x (.Origin (Collision|GetActorBounds (stale EventBeginPlay _output_get) false false))) (.y (.Origin (Collision|GetActorBounds (stale EventBeginPlay _output_get) false false))) (- (.z (.Origin (Collision|GetActorBounds (stale EventBeginPlay _output_get) false false))) 1e+02)))) (.yaw (Math|Rotator|FindLookatRotation (Transformation|GetWorldLocation __leftarrow) (Math|Vector|MakeVector (.x (.Origin (Collision|GetActorBounds (stale EventBeginPlay _output_get) false false))) (.y (.Origin (Collision|GetActorBounds (stale EventBeginPlay _output_get) false false))) (- (.z (.Origin (Collision|GetActorBounds (stale EventBeginPlay _output_get) false false))) 1e+02))))) false false))
    (:then_1
      (Transformation|SetWorldRotation __righttarrow (Math|Rotator|FindLookatRotation (Transformation|GetWorldLocation __righttarrow) (Math|Vector|MakeVector (.x (.Origin (Collision|GetActorBounds (stale EventBeginPlay _output_get) false false))) (.y (.Origin (Collision|GetActorBounds (stale EventBeginPlay _output_get) false false))) (- (.z (.Origin (Collision|GetActorBounds (stale EventBeginPlay _output_get) false false))) 1e+02))) false false))))

(event EventBeginPlay
  (bind _asbp_character (Utilities|Casting|CastToBP_Character (Game|GetPlayerCharacter 0)))
  (bind _output_get (Variables|Default|SetAs%20BP%20Character _asbp_character)))

(fn ConstructionScript)