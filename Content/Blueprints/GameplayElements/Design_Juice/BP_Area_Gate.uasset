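; BP_Area_Gate is a gate actor that swings open and has a light or dark look.
; BeginPlay stores the Arrow component's starting rotation and a target offset in yaw by RotationAmount.
; OpenGate plays a timeline that lerps the Arrow between those rotations.
; The construction script picks the light or dark gate material from the Light flag.
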(event Custom|Open%20Gate
  (bind _alpha (Timeline|T_Rotate Play)
    (:Update
      (Transformation|SetRelativeRotation (Variables|Default|GetArrow) (Math|Rotator|Lerp(Rotator) (Variables|Default|GetStarting%20Rotation) (Variables|Default|GetTarget%20Rotation) _alpha) false false))))

(event EventBeginPlay
  (bind _output_get (Variables|Default|SetStarting%20Rotation (Variables|/Script/Engine.SceneComponent|GetRelativeRotation (Variables|Default|GetArrow))))
  (Variables|Default|SetTarget%20Rotation (Math|Rotator|MakeRotator (.roll _output_get) (.pitch _output_get) (+ (.yaw _output_get) (Variables|Default|GetRotation%20Amount)))))

(fn ConstructionScript
  (bind _gate (Variables|Default|GetGate))
  (if (Variables|Default|GetLight?)
    (Rendering|Material|SetMaterial _gate 0 "/Game/Assets/Meshes/Gate_Assets/light_v1/M_Gate_Light.M_Gate_Light")
    (else
      (Rendering|Material|SetMaterial _gate 0 "/Game/Assets/Meshes/Gate_Assets/dark_v2/M_Gate_Dark.M_Gate_Dark"))))