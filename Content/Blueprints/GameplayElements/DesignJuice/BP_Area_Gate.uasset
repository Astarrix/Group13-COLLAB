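; BP_Area_Gate is a gate actor that swings open once when the Area Manager calls OpenGate.
; On BeginPlay it stores the Arrow component's rotation and derives a target by adding RotationAmount to yaw.
; A DoOnce-guarded timeline lerps the Arrow between those rotations, printing debug messages at start and finish.
; The construction script picks a light or dark gate material from the Light flag.
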(event Custom|Open%20Gate
  ;[1 1 1] Open gate when called from Area Manager
  (Utilities|FlowControl|DoOnce false
    (:Completed
      (Development|PrintString "Gate opening" true true "(R=0.085358,G=1.000000,B=0.000000,A=1.000000)" 25.0 "Gate")
      (bind _alpha (Timeline|T_Rotate Play)
        (:Update
          (Transformation|SetRelativeRotation (Variables|Default|GetArrow) (Math|Rotator|Lerp(Rotator) (Variables|Default|GetStarting%20Rotation) (Variables|Default|GetTarget%20Rotation) _alpha) false false))
        (:Finished
          (Development|PrintString "Gate fullyed opened!" true true "(R=1.000000,G=0.235914,B=0.000000,A=1.000000)" 5.0 "Gate"))))))

(event EventBeginPlay
  ;[1 1 1] Init rotation amount
  (bind _output_get (Variables|Default|SetStarting%20Rotation (Variables|/Script/Engine.SceneComponent|GetRelativeRotation (Variables|Default|GetArrow))))
  (Variables|Default|SetTarget%20Rotation (Math|Rotator|MakeRotator (.roll _output_get) (.pitch _output_get) (+ (.yaw _output_get) (Variables|Default|GetRotation%20Amount)))))

(fn ConstructionScript
  (bind _gate (Variables|Default|GetGate))
  (if (Variables|Default|GetLight?)
    (Rendering|Material|SetMaterial _gate 0 "/Game/Assets/Meshes/Gate_Assets/light_v1/M_Gate_Light.M_Gate_Light")
    (else
      (Rendering|Material|SetMaterial _gate 0 "/Game/Assets/Meshes/Gate_Assets/dark_v2/M_Gate_Dark.M_Gate_Dark"))))