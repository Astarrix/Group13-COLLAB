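; BP_TargetWindowV2 is a gameplay-element actor for a target window, built with a large set of Box components that serve as its window colliders.
; ReturnWindowColliders hands those boxes back as a hand-assembled array, giving callers a single access point to the colliders.
; It has no other logic of its own: the event stubs are disabled and the construction script only calls its parent.
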(event EventBeginPlay
  (|CallParentFunction) ; This node is disabled and will not be called.\nDrag off pins to build functionality.
)

(event Collision|EventActorBeginOverlap
  (params (OtherActor :type Actor%20Object%20Reference)))

(event EventTick
  (params (DeltaSeconds :type Float%20%28single-precision%29)))

(fn ConstructionScript
  (|CallParentFunction))

(fn ReturnWindowColliders
  (return (Utilities|Array|MakeArray (Variables|Default|GetBox14) (Variables|Default|GetBox23) (Variables|Default|GetBox22) (Variables|Default|GetBox21) (Variables|Default|GetBox20) (Variables|Default|GetBox25) (Variables|Default|GetBox30) (Variables|Default|GetBox29) (Variables|Default|GetBox28) (Variables|Default|GetBox27) (Variables|Default|GetBox26) (Variables|Default|GetBox19) (Variables|Default|GetBox11) (Variables|Default|GetBox10) (Variables|Default|GetBox12) (Variables|Default|GetBox9) (Variables|Default|GetBox8) (Variables|Default|GetBox18) (Variables|Default|GetBox17) (Variables|Default|GetBox16) (Variables|Default|GetBox13) (Variables|Default|GetBox15) (Variables|Default|GetBox24) (Variables|Default|GetBox31) (Variables|Default|GetBox48) (Variables|Default|GetBox47) (Variables|Default|GetBox46) (Variables|Default|GetBox45) (Variables|Default|GetBox49) (Variables|Default|GetBox44) (Variables|Default|GetBox51) (Variables|Default|GetBox50) (Variables|Default|GetBox36) (Variables|Default|GetBox35) (Variables|Default|GetBox34) (Variables|Default|GetBox33) (Variables|Default|GetBox32) (Variables|Default|GetBox37) (Variables|Default|GetBox43) (Variables|Default|GetBox42) (Variables|Default|GetBox41) (Variables|Default|GetBox40) (Variables|Default|GetBox39) (Variables|Default|GetBox38))))