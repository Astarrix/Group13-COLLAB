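; Tutorial spline actor that drives a van along a path to successive target locations.
; NextLocationActivated scales a timeline to the requested travel time, lerping spline distance from the previous location to the new one.
; The first actor in ActorsToMove follows the spline's position and rotation, with yaw flipped 180 degrees.
; The construction script snaps spline points to the floor with line traces and moves a visible Box to the last point.
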(event Custom|NextLocationActivated
  (params (NewVanLocation :type Transform) (TimeToLocation :type Float%20%28double-precision%29%20%28by%20ref%29))
  (bind _location (Math|Transform|BreakTransform NewVanLocation))
  (bind _splinedecalplacer (Variables|Default|GetSplineDecalPlacer))
  ;[1 1 1] Move van to next location
  (Components|Timeline|SetPlayRate (Variables|Default|GetT_MoveVan) (/ 1.0 TimeToLocation))
  (bind _t_movevan (Timeline|T_MoveVan PlayFromStart)
    (:Update
      (Transformation|SetActorTransform (Utilities|Array|Get(acopy) (Variables|Default|GetActorsToMove)) (Math|Transform|MakeTransform (Spline|GetLocationatDistanceAlongSpline _splinedecalplacer (Math|Float|Lerp (Class|SplineComponent|GetDistanceAlongSplineatLocation _splinedecalplacer (Variables|Default|GetPrevious%20Location) "World") (Class|SplineComponent|GetDistanceAlongSplineatLocation _splinedecalplacer _location "World") _t_movevan) "World") (Math|Rotator|MakeRotator (.roll (Spline|GetRotationatDistanceAlongSpline _splinedecalplacer (Math|Float|Lerp (Class|SplineComponent|GetDistanceAlongSplineatLocation _splinedecalplacer (Variables|Default|GetPrevious%20Location) "World") (Class|SplineComponent|GetDistanceAlongSplineatLocation _splinedecalplacer _location "World") _t_movevan) "World")) (.pitch (Spline|GetRotationatDistanceAlongSpline _splinedecalplacer (Math|Float|Lerp (Class|SplineComponent|GetDistanceAlongSplineatLocation _splinedecalplacer (Variables|Default|GetPrevious%20Location) "World") (Class|SplineComponent|GetDistanceAlongSplineatLocation _splinedecalplacer _location "World") _t_movevan) "World")) (+ (.yaw (Spline|GetRotationatDistanceAlongSpline _splinedecalplacer (Math|Float|Lerp (Class|SplineComponent|GetDistanceAlongSplineatLocation _splinedecalplacer (Variables|Default|GetPrevious%20Location) "World") (Class|SplineComponent|GetDistanceAlongSplineatLocation _splinedecalplacer _location "World") _t_movevan) "World")) 1.8e+02)) "1.000000,1.000000,1.000000")))
    (:Finished
      (Variables|Default|SetPrevious%20Location _location))))

(event EventBeginPlay
  ;[1 1 1] Init set starting van location
  (Variables|Default|SetPrevious%20Location (Transformation|GetActorLocation)))

(fn ConstructionScript
  (bind _splinedecalplacer (Variables|Default|GetSplineDecalPlacer))
  (bind _box (Variables|Default|GetBox))
  (bind _splinedecalplacer_2 (Variables|Default|GetSplineDecalPlacer))
  (bind _returnvalue (Spline|GetNumberOfSplinePoints _splinedecalplacer))
  (bind _returnvalue_2 (- _returnvalue 1))
  (Utilities|FlowControl|Sequence
    (:then_0
      ;[1 0 0] Snap Spline Points To Floor
      (for _index (range 0 _returnvalue_2)
        (bind (_outhit _returnvalue_3) (Collision|LineTraceByChannel (Math|Vector|MakeVector (.x (Spline|GetLocationatSplinePoint _splinedecalplacer_2 _index "World")) (.y (Spline|GetLocationatSplinePoint _splinedecalplacer_2 _index "World")) (+ (.z (Spline|GetLocationatSplinePoint _splinedecalplacer_2 _index "World")) (Variables|DecalSplineSetup|GetDecalSnapOffset))) (Math|Vector|MakeVector (.x (Spline|GetLocationatSplinePoint _splinedecalplacer_2 _index "World")) (.y (Spline|GetLocationatSplinePoint _splinedecalplacer_2 _index "World")) (- (.z (Spline|GetLocationatSplinePoint _splinedecalplacer_2 _index "World")) (Variables|DecalSplineSetup|GetDecalSnapOffset))) "TraceTypeQuery1" false 0 "ForDuration" true "(R=1.000000,G=0.000000,B=0.000000,A=1.000000)" "(R=0.000000,G=1.000000,B=0.000000,A=1.000000)" 2.0))
        (if _returnvalue_3
          (Spline|SetLocationatSplinePoint (Variables|Default|GetSplineDecalPlacer) _index (.location _outhit) "World" true)
          (Transformation|SetWorldLocation _box (Spline|GetLocationatSplinePoint (Variables|Default|GetSplineDecalPlacer) _returnvalue_2 "World") false true)
          (Development|SetHiddeninGame _box false false))))))