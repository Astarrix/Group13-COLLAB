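; Base pickup actor that destroys itself when an overlapping actor successfully picks it up.
; Sphere overlaps call ObjectPickedUp, which returns false here, leaving pickup logic to child Blueprints.
; The construction script recenters any mesh from its bounds and sizes the collision sphere to match.
; A timeline started on BeginPlay drives a vertical bounce, while the collision-delay logic is unconnected and never runs.
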(event OnComponentBeginOverlap(Collision)
  (params (OverlappedComponent :type Primitive%20Component%20Object%20Reference) (OtherActor :type Actor%20Object%20Reference) (OtherComp :type Primitive%20Component%20Object%20Reference) (OtherBodyIndex :type Integer) (bFromSweep :type Boolean) (SweepResult :type Hit%20Result%20Structure%20%28by%20ref%29))
  (bind _isdestroyed (CallFunction|ObjectPickedUp OtherActor))
  (if _isdestroyed
    (Actor|DestroyActor)))

(event EventBeginPlay
  (Components|Timeline|SetPlayRate (Variables|Default|GetBounce) 2.0)
  (bind _bouncetrack (Timeline|Bounce PlayFromStart)
    (:Update
      (Transformation|SetRelativeLocation (Math|Vector|MakeVector 0.0 0.0 (Math|Float|Lerp 0.0 1e+02 _bouncetrack)) false false))))

(fn ConstructionScript
  (bind _pickupmesh (Variables|Default|GetPickupMesh))
  (bind _collision (Variables|Default|GetCollision))
  (bind _staticmesh (Variables|/Script/Engine.StaticMeshComponent|GetStaticMesh _pickupmesh))
  (bind _returnvalue (StaticMesh|GetBounds _staticmesh))
  (bind (_origin _boxextent _sphereradius) (Math|BoxSphereBounds|BreakBoxSphereBounds _returnvalue))
  ;[0.01938 0.4969 1] Recenters mesh agnostic to import
  (Transformation|SetRelativeLocation (Variables|Default|GetPickupMesh) (+ (* _origin "-1.000000,-1.000000,-1.000000") (Math|Vector|MakeVector 0.0 0.0 (.Z (Math|Vector|BreakVector _boxextent)))) false false)
  ;[0.3564 0.04092 0.521] Resize & Reposition Collision
  (Transformation|SetRelativeLocation _collision "0, 0, 0" false false)
  (Components|Sphere|SetSphereRadius _collision _sphereradius false)
  (Transformation|SetRelativeLocation "0, 0, 0" false false))

(fn ObjectPickedUp
  (params (CollidingActor :type Actor%20Object%20Reference))
  (return false))