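; Shop item for purchasable player stat upgrades, typed as spray radius or movement speed, extending a parent shop item class.
; Construction sets the mesh from the upgrade type, though both types use the Squeegee.
; BeginPlay caches the player's BP_Character, and interaction defers to the parent.
; Purchasing handles only the Spray Radius case, which raises the character's max walk speed by a fixed amount and returns false.
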(event EventBeginPlay
  (|CallParentFunction)
  (bind _asbp_character (Utilities|Casting|CastToBP_Character (Game|GetPlayerCharacter 0)))
  (Variables|Default|SetAs%20BP%20Character _asbp_character))

(event Collision|EventActorBeginOverlap
  (params (OtherActor :type Actor%20Object%20Reference)))

(event EventTick
  (params (DeltaSeconds :type Float%20%28single-precision%29)))

(fn ConstructionScript
  (|CallParentFunction)
  (Components|StaticMesh|SetStaticMesh (Variables|Default|GetStaticMesh) (Utilities|Select :Index (Variables|Default|GetUpgradeType) :NewEnumerator0 "/Game/Assets/Rig/squeegee.squeegee" :NewEnumerator1 "/Game/Assets/Rig/squeegee.squeegee")))

(fn Interactedwith
  (|CallParentFunction))

(fn Purchased
  (bind _as_bp_character (Variables|Default|GetAs%20BP%20Character))
  (bind _charactermovement (Variables|/Script/Engine.Character|GetCharacterMovement _as_bp_character))
  (switch Utilities|FlowControl|Switch|SwitchoneStatUpgradeType (Variables|Default|GetUpgradeType)
    (:NewEnumerator0
      (Variables|/Script/Engine.CharacterMovementComponent|SetMaxWalkSpeed _charactermovement (+ (Variables|/Script/Engine.CharacterMovementComponent|GetMaxWalkSpeed _charactermovement) 5e+01))
      (return false))))