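; Shop item that sells an arm by spawning an arm pickup in the world when purchased.
; The construction script previews the item by reading the arm mesh from the SpawnedClass defaults, then runs the parent construction script.
; Purchased spawns a BP_ArmPickup at SpawnLocation, passing the arm class and left-arm flag, and always returns true.
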(fn ConstructionScript
  (Components|StaticMesh|SetStaticMesh (.ArmMesh (Utilities|GetClassDefaults (Variables|Default|GetSpawnedClass))))
  (|CallParentFunction))

(fn Purchased
  (Game|SpawnActorfromClass "/Game/Blueprints/GameplayElements/Weapons/BP_ArmPickup.BP_ArmPickup_C" (Math|Transform|MakeTransform (Variables|Default|GetSpawnLocation)) "AdjustIfPossibleButAlwaysSpawn" "MultiplyWithRoot" 0 (Variables|Default|GetIs%20Left%20Arm) (Variables|Default|GetSpawnedClass) 0)
  (return true))