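; BP_Van is a shop van whose shutter opens when the player approaches and closes when they leave.
; A sphere overlap plays or reverses a timeline that rotates the shutter pivot, with a DoOnce gating its sound.
; On BeginPlay, a box overlap finds nearby BP_ShopItem_Spawn actors and gives them the van's spawn location.
; Looking at the van enables input for opening a LevelSwitch UI widget; looking away removes it.
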(event OnComponentBeginOverlap(Sphere)
  (params (OverlappedComponent :type Primitive%20Component%20Object%20Reference) (OtherActor :type Actor%20Object%20Reference) (OtherComp :type Primitive%20Component%20Object%20Reference) (OtherBodyIndex :type Integer) (bFromSweep :type Boolean) (SweepResult :type Hit%20Result%20Structure%20%28by%20ref%29))
  ;[1 1 1] Makes It only open for player and stays open
  (if (== (Game|GetPlayerCharacter 0) OtherActor)
    (bind _shutterrotation (Timeline|ShutterRotation Play)
      (:Update
        (Transformation|SetRelativeRotation (Variables|Default|GetShutterPivotPoint) (Math|Rotator|MakeRotator (Math|Float|Lerp 0.0 -7e+01 _shutterrotation) 0.0 0.0) false false)
        ;[0.9424 0.2266 1] Shutter Noise
        (Utilities|FlowControl|DoOnce false :!label _label
          (:Completed
            (Audio|PlaySoundatLocation "/Game/Audio/SFXs/Van_ShutterNoise.Van_ShutterNoise" (Transformation|GetWorldLocation (Variables|Default|GetDefaultSceneRoot)) "0, 0, 0" 1.0 1.0 0.5 0 0 0 0))))
      (:Finished
        (goto _label Reset)))))

(event OnComponentEndOverlap(Sphere)
  (params (OverlappedComponent :type Primitive%20Component%20Object%20Reference) (OtherActor :type Actor%20Object%20Reference) (OtherComp :type Primitive%20Component%20Object%20Reference) (OtherBodyIndex :type Integer))
  ;[1 1 1] Makes It only open for player and stays open
  (if (== OtherActor (Game|GetPlayerCharacter 0))
    (bind _shutterrotation (Timeline|ShutterRotation Reverse)
      (:Update
        (Transformation|SetRelativeRotation (Variables|Default|GetShutterPivotPoint) (Math|Rotator|MakeRotator (Math|Float|Lerp 0.0 -7e+01 _shutterrotation) 0.0 0.0) false false)
        ;[0.9424 0.2266 1] Shutter Noise
        (Utilities|FlowControl|DoOnce false :!label _label
          (:Completed
            (Audio|PlaySoundatLocation "/Game/Audio/SFXs/Van_ShutterNoise.Van_ShutterNoise" (Transformation|GetWorldLocation (Variables|Default|GetDefaultSceneRoot)) "0, 0, 0" 1.0 1.0 0.5 0 0 0 0))))
      (:Finished
        (goto _label Reset)))))

(event Custom|NextLocation)

(event Custom|LinkItems
  (bind _outactors (Collision|BoxOverlapActors (Transformation|GetActorLocation) "1000.000000,1000.000000,1000.000000" (Utilities|Array|MakeArray "ObjectTypeQuery1" "ObjectTypeQuery2") "/Game/Blueprints/GameplayElements/Shop/BP_ShopItem.BP_ShopItem_C" :!class /Script/Engine.KismetSystemLibrary))
  (bind _filteredarray (Utilities|Array|FilterArray _outactors "/Game/Blueprints/GameplayElements/Shop/BP_ShopItem.BP_ShopItem_C"))
  (for _array_element _filteredarray
    (bind _asbp_shop_item_spawn (Utilities|Casting|CastToBP_ShopItem_Spawn _array_element))
    (Variables|/Game/Blueprints/GameplayElements/Shop/BP_ShopItem_Spawn.BP_ShopItem_Spawn_C|SetSpawnLocation _asbp_shop_item_spawn (Transformation|GetWorldLocation (Variables|Default|GetSpawnLocation)))))

(event Input|EnhancedActionEvents|EnhancedInputActionIA_LeftArmActivate
  (params (ActionValue :type Boolean) (ElapsedSeconds :type Float%20%28double-precision%29) (TriggeredSeconds :type Float%20%28double-precision%29) (InputAction :type Input%20Action%20Object%20Reference :default "/Game/Input/InputActions/IA_LeftArmActivate.IA_LeftArmActivate"))
  (bind _returnvalue (Game|GetPlayerController 0))
  (:Started
    (bind _returnvalue_2 (UserInterface|CreateWidget "/Game/UI/MainMenu/NewWidgetBlueprint.NewWidgetBlueprint_C"))
    (bind _output_get (Variables|Default|SetLevelSwitch _returnvalue_2))
    (Input|SetInputModeUIOnly _returnvalue _output_get "DoNotLock" false)
    (UserInterface|Viewport|AddtoViewport _output_get 0)
    (Variables|/Script/Engine.PlayerController|SetbShowMouseCursor _returnvalue true)))

(event EventBeginPlay
  (CallFunction|LinkItems))

(event EventLookedat
  (Input|EnableInput (Game|GetPlayerController 0)))

(event EventStopLookat
  (bind _returnvalue (Game|GetPlayerController 0))
  (Input|DisableInput _returnvalue)
  (bind _levelswitch (Variables|Default|GetLevelSwitch)
    (:then
      (Widget|RemovefromParent _levelswitch)
      (Input|SetInputModeGameOnly _returnvalue false)
      (Variables|/Script/Engine.PlayerController|SetbShowMouseCursor _returnvalue false))
    (:else)))

(fn ConstructionScript)