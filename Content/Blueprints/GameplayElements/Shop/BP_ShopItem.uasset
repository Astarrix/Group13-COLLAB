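; Base shop item that the player can inspect and buy with the character's money.
; The construction script uniformly scales its mesh from its bounds and a maximum item height.
; Looking at it broadcasts name, description and price, which also fill the on-screen UI text.
; Interacting deducts the price if affordable, calls Purchased (a stub returning false here) and completes any assigned objective task.
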(event EventLookedat
  (|CallParentFunction)
  (Default|CallOnLookedat (Variables|Default|GetItem%20Name) (Variables|Default|GetItem%20Description) (Variables|Default|GetItem%20Price)))

(fn ConstructionScript
  (bind _staticmesh (Variables|Default|GetStaticMesh))
  (bind _maxitemheight (Variables|Default|GetMaxItemHeight))
  (bind _staticmesh_2 (Variables|/Script/Engine.StaticMeshComponent|GetStaticMesh _staticmesh))
  (bind _returnvalue (StaticMesh|GetBounds _staticmesh_2))
  (bind _boxextent (Math|BoxSphereBounds|BreakBoxSphereBounds _returnvalue))
  (bind _z (Math|Vector|BreakVector _boxextent))
  (bind _returnvalue_2 (/ _maxitemheight _z))
  (|CallParentFunction)
  (Transformation|SetRelativeScale3D _staticmesh (Math|Vector|MakeVector _returnvalue_2 _returnvalue_2 _returnvalue_2)))

(fn Interactedwith
  (bind _returnvalue (Game|GetPlayerCharacter 0))
  (bind _item_price (Variables|Default|GetItem%20Price))
  (bind _objectivetaskid (Variables|Default|GetObjectiveTaskID))
  (bind _asbp_character (Utilities|Casting|CastToBP_Character _returnvalue))
  (if (>= (Variables|/Game/Blueprints/Core/BP_Character.BP_Character_C|GetMoney _asbp_character) _item_price)
    (Default|ChangeMoney _asbp_character (* _item_price -1))
    (bind _isconsumedonpurchase (CallFunction|Purchased))
    (if (!= _objectivetaskid "")
      (CallFunction|MarkObjectiveasComplete _objectivetaskid))
    (return _isconsumedonpurchase)
    (else
      (return false))))

(fn Purchased
  (return false))

(fn AddonScreenUI
  (return (Class|KismetTextLibrary|TexttoUpper (Variables|Default|GetItem%20Name)) (Utilities|Text|FormatText "{desc} 
Cost: {p}" (Variables|Default|GetItem%20Description) (Variables|Default|GetItem%20Price))))