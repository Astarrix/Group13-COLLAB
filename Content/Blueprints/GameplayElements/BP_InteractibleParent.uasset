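; BP_InteractibleParent is the base actor for objects the player can look at and interact with.
; On BeginPlay it sets the mesh's custom-depth stencil and creates a hidden key prompt widget showing a configurable key image.
; Lookedat and StopLookat toggle the outline depth pass, prompt and player input.
; IA_Interact calls InteractedWith, which returns false here for children to override, and destroys the actor on true.
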(event Input|EnhancedActionEvents|EnhancedInputActionIA_Interact
  (params (ActionValue :type Boolean) (ElapsedSeconds :type Float%20%28double-precision%29) (TriggeredSeconds :type Float%20%28double-precision%29) (InputAction :type Input%20Action%20Object%20Reference :default "/Game/Input/InputActions/IA_Interact.IA_Interact"))
  (:Started
    (bind _isdestroyed (CallFunction|Interactedwith))
    (if _isdestroyed
      (Actor|DestroyActor)
      (Widget|SetVisibility (Variables|Default|GetOnScreenPrompt) "Hidden"))))

(event EventLookedat
  (Rendering|SetRenderCustomDepth (Variables|Default|GetStaticMesh) true)
  (Input|EnableInput (Game|GetPlayerController 0))
  (Widget|SetVisibility (Variables|Default|GetOnScreenPrompt) "HitTestInvisible"))

(event EventStopLookat
  (Rendering|SetRenderCustomDepth (Variables|Default|GetStaticMesh) false)
  (Input|DisableInput (Game|GetPlayerController 0))
  (Widget|SetVisibility (Variables|Default|GetOnScreenPrompt) "Hidden"))

(event EventBeginPlay
  (Rendering|SetCustomDepthStencilValue (Variables|Default|GetStaticMesh) (Variables|Default|GetColourMask))
  (bind _returnvalue (UserInterface|CreateWidget "/Game/UI/Tutorialisation/WBP_KeyPrompt.WBP_KeyPrompt_C"))
  (Appearance|SetBrushfromTexture (Variables|/Game/UI/Tutorialisation/WBP_KeyPrompt.WBP_KeyPrompt_C|GetIMG_KeyToShow _returnvalue) (Variables|Default|GetKeyToShow) false)
  (UserInterface|Viewport|AddtoPlayerScreen _returnvalue)
  (bind _output_get (Variables|Default|SetOnScreenPrompt _returnvalue))
  (Widget|SetVisibility _output_get "Hidden"))

(fn ConstructionScript)

(fn Interactedwith
  (return false))