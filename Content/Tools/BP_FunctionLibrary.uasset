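; Blueprint function library with helpers for camera shakes, curve sampling and integer bit math.
; CameraShakeWithOptions packs an FOV flag and pitch, yaw and roll levels into bit fields, passed through the Scale of a BP_CameraShakeManager legacy shake.
; Shifts multiply by looped integer powers, though RightBitShift uses base -2, so it doesn't truly shift right.
; LinearValueToCurve samples a float curve at a Min–Max normalized input.
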(fn LinearValuetoCurve
  (params (Target :type Curve%20Float%20Object%20Reference) (InTime :type Float%20%28single-precision%29) (Min :type Float%20%28double-precision%29) (Max :type Float%20%28double-precision%29))
  (return (Math|Curves|GetFloatValue Target (/ (- InTime Min) (- Max Min)))))

(fn CameraShakewithOptions
  (params (PlayerCameraManager :type Player%20Camera%20Manager%20Object%20Reference) (isFOVShake :type Boolean) (PitchScale%20%280-7%29 :type Integer) (YawScale%20%280-7%29 :type Integer) (RollScale%20%280.7%29 :type Integer))
  (Class|LegacyCameraShake|StartLegacyCameraShake PlayerCameraManager "/Game/Blueprints/BP_CameraShakeManager.BP_CameraShakeManager_C" (Math|Conversions|ToFloat(Integer) (+ (Math|Conversions|ToInteger(Boolean) isFOVShake) (CallFunction|LeftBitShift PitchScale%20%280-7%29 1) (CallFunction|LeftBitShift YawScale%20%280-7%29 4) (CallFunction|LeftBitShift RollScale%20%280.7%29 7))) "CameraLocal" "0, 0, 0")
  (return))

(fn LeftBitShift
  (params (Data :type Integer) (Positions :type Integer))
  (return (* Data (CallFunction|Power(Int) 2 Positions))))

(fn Power(Int)
  (params (Base :type Integer) (Exponent :type Integer))
  (LocalVariables|SetCarry 1)
  (for _index (range 1 Exponent)
    (LocalVariables|SetCarry (* (LocalVariables|GetCarry) Base)))
  (return (LocalVariables|GetCarry)))

(fn RightBitShift
  (params (Data :type Integer) (Positions :type Integer))
  (return (* Data (CallFunction|Power(Int) -2 Positions))))